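; Player controller for a turn-based, grid-based survivors-versus-zombies game that turns mouse and keyboard input into survivor actions.
; Left click selects a survivor, move target or shot by control mode, using cursor line traces passed to the GridManager.
; Space commits moves and looting or ends the zombie turn, and H heals, all through the GameManager and disabled after game end.
; Move mode feeds the active survivor's range and cell to the grid.
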(event Custom|SelectSurvivorMoveTarget
  ;[1 1 1] Shoots Raycast to mouse position and triggers grid movement
  (bind (_point _istherehit) (CallFunction|TracetoMousePosition))
  (if _istherehit
    (Default|OnPlayerCellSelection (Variables|Default|GetGridMangerRef) _point)))

(event Custom|GameStarted
  (Variables|Default|SetgameEnded false))

(event Custom|TriggerShoot
  ;[1 1 1] GetPosition of cell to shoot from
  (bind (_point _istherehit) (CallFunction|TracetoMousePosition))
  (if _istherehit
    (Default|SurvivorShoot (Variables|Default|GetGridMangerRef) _point)))

(event Custom|GivePlayerData
  (bind _gridmangerref (Variables|Default|GetGridMangerRef))
  (bind _gamemanager (Variables|Default|GetGameManager))
  (bind _activesurvivorref (Variables|/Game/Blueprints/Student/Blueprints/GameManagement/GameManager.GameManager_C|GetActiveSurvivorRef _gamemanager))
  ;[1 1 1] Get cell character is on
  (Utilities|IsValid _activesurvivorref
    (:Is%20Valid
      (bind (_array_index _cellexist) (Default|GetCellwithCharacter (Variables|Default|GetGridMangerRef) _activesurvivorref))
      (if _cellexist
        (bind _cellcoordinate (Default|GetCellCoordinate _gridmangerref _array_index))
        ;[1 1 1] Pass in survivor range and coordinate
        (Default|SetCurrentSurvivorData _gridmangerref (Variables|/Game/Blueprints/Student/Blueprints/Characters/BP_BaseCharacter.BP_BaseCharacter_C|GetmaxSteps _activesurvivorref) _cellcoordinate)))))

(event EventBeginPlay
  ;[1 1 1] Cache actor references
  (bind _returnvalue (Actor|GetActorOfClass "/Game/Blueprints/B_AdvCharacter.B_AdvCharacter_C"))
  (Variables|Default|SetCharacterRef _returnvalue)
  (bind _returnvalue_2 (Actor|GetActorOfClass "/Game/Blueprints/Student/Blueprints/Grid/BP_GridManager.BP_GridManager_C"))
  (Variables|Default|SetGridMangerRef _returnvalue_2)
  (bind _returnvalue_3 (Actor|GetActorOfClass "/Game/Blueprints/Student/Blueprints/GameManagement/GameManager.GameManager_C"))
  (bind _output_get (Variables|Default|SetGameManager _returnvalue_3))
  (EventDispatchers|BindEventtoOnEndGame _output_get (delegate EventEndGame))
  (EventDispatchers|BindEventtoOnStartGame _output_get (delegate Custom|GameStarted)))

(event EventEndGame
  (Variables|Default|SetgameEnded true))

(event Input|KeyboardEvents|SpaceBar
  (params (Key :type Key%20Structure :default "None"))
  (bind _gamemanager (Variables|Default|GetGameManager))
  ;[1 1 1] Commit action key
  (:Pressed
    (if (not (Variables|Default|GetgameEnded))
      (switch Utilities|FlowControl|Switch|SwitchonTurnState (Variables|/Game/Blueprints/Student/Blueprints/GameManagement/GameManager.GameManager_C|GetcurrentTurn _gamemanager)
        (:NewEnumerator0
          (switch Utilities|FlowControl|Switch|SwitchonControlMode (Variables|Default|GetcurrentMode)
            (:NewEnumerator0
              (Default|MoveCharacter (Variables|Default|GetGameManager)))
            (:NewEnumerator2
              (Default|SurvivorLoot (Variables|Default|GetGameManager)))))
        (:NewEnumerator1
          (Default|EndZombieTurn _gamemanager))))))

(event Input|MouseEvents|LeftMouseButton
  (params (Key :type Key%20Structure :default "None"))
  (bind _gamemanager (Variables|Default|GetGameManager))
  (bind _activesurvivorref (Variables|/Game/Blueprints/Student/Blueprints/GameManagement/GameManager.GameManager_C|GetActiveSurvivorRef _gamemanager))
  ;[1 1 1] Click events
  (:Pressed
    (if (not (Variables|Default|GetgameEnded))
      (switch Utilities|FlowControl|Switch|SwitchonTurnState (Variables|/Game/Blueprints/Student/Blueprints/GameManagement/GameManager.GameManager_C|GetcurrentTurn (Variables|Default|GetGameManager))
        (:NewEnumerator0
          (switch Utilities|FlowControl|Switch|SwitchonControlMode (Variables|Default|GetcurrentMode)
            (:NewEnumerator0
              (CallFunction|SelectSurvivorMoveTarget))
            (:NewEnumerator1
              (CallFunction|TriggerShoot))
            (:NewEnumerator3
              (CallFunction|SelectSurvivor)
              (Utilities|IsValid _activesurvivorref
                (:Is%20Valid
                  (EventDispatchers|BindEventtoOnActionEnd _activesurvivorref (delegate Custom|GivePlayerData)))))))))))

(event Input|KeyboardEvents|H
  (params (Key :type Key%20Structure :default "None"))
  (:Pressed
    ;[1 1 1] Heal Character
    (if (not (Variables|Default|GetgameEnded))
      ;[1 1 1] Only on player turn
      (switch Utilities|FlowControl|Switch|SwitchonTurnState (Variables|/Game/Blueprints/Student/Blueprints/GameManagement/GameManager.GameManager_C|GetcurrentTurn (Variables|Default|GetGameManager))
        (:NewEnumerator0
          (Default|HealActiveSurvivor (Variables|Default|GetGameManager)))))))

(fn ConstructionScript)

(fn TracetoMousePosition
  (bind _returnvalue (Game|GetPlayerController 0))
  (bind (_worldlocation _worlddirection) (Game|Player|ConvertMouseLocationToWorldSpace _returnvalue))
  (bind (_outhit _returnvalue_2) (Collision|LineTraceByChannel _worldlocation (+ _worldlocation (* _worlddirection (Variables|Default|GetTraceLength))) "TraceTypeQuery1" false 0 "None"))
  (if _returnvalue_2
    (return (.ImpactPoint (Collision|BreakHitResult _outhit)) _returnvalue_2)
    (else
      (Development|PrintString "Hit Nothing"))))

(fn ChangeMode
  (bind _result (Math|Integer|IncrementInt (Math|Conversions|ToInteger(Byte) (Variables|Default|GetcurrentMode)))
    (:%20%20
      (if (< _result (|GetNumEnumEntries))
        (Variables|Default|SetcurrentMode (Utilities|Enum|ByteToEnumControlMode (Math|Conversions|ToByte(Integer) _result)))
        (else
          (Variables|Default|SetcurrentMode "NewEnumerator0"))))))

(fn TracetoCharacter
  (bind (_worldlocation _worlddirection) (Game|Player|ConvertMouseLocationToWorldSpace))
  ;[1 1 1] Comment
  (bind (_outhit _returnvalue) (Collision|LineTraceByChannel _worldlocation (+ _worldlocation (* _worlddirection (Variables|Default|GetTraceLength))) "TraceTypeQuery1" false 0 "None"))
  (if _returnvalue
    (if (== (Utilities|GetClass (.HitActor (Collision|BreakHitResult _outhit))) "/Game/Blueprints/Student/Blueprints/Characters/BP_BaseSurvivor.BP_BaseSurvivor_C")
      (bind _asbp_base_survivor (Utilities|Casting|CastToBP_BaseSurvivor (.HitActor (Collision|BreakHitResult _outhit))))
      (return _asbp_base_survivor true)
      (else
        (return 0 false)))))

(fn SetControlMode
  (params (currentMode :type ControlMode%20Enum :default "NewEnumerator0"))
  (bind _output_get (Variables|Default|SetcurrentMode currentMode))
  (switch Utilities|FlowControl|Switch|SwitchonControlMode _output_get
    (:NewEnumerator0
      (CallFunction|GivePlayerData))))

(fn SelectSurvivor
  (Default|UnselectActiveCharacter (Variables|Default|GetGameManager))
  (bind _asbase_survivor (CallFunction|TracetoCharacter))
  (Utilities|IsValid _asbase_survivor
    (:Is%20Valid
      (Default|SetActiveSurvivor (Variables|Default|GetGameManager) _asbase_survivor)
      (Default|SelectActiveCharacter (Variables|Default|GetGameManager)))))