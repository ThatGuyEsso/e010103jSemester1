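; Base character that moves across a GridManager's cells and keeps the GridFloor occupancy flags in sync with its position.
; The construction script finds the GridManager, and BeginPlay marks the starting cell as occupied.
; MoveToGridPoint frees the current cell and lerps location on a timeline, updating the grid index as it goes.
; On finish it clears the cell's floor and target states, marks it occupied, then calls itself for the next point stored by SetPath.
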(event Custom|MoveToGridPoint
  (params (newPoint :type Vector) (startPoint :type Vector))
  (bind _returnvalue (Transformation|GetActorLocation))
  (bind _gridmanagerref (Variables|Default|GetGridManagerRef))
  (bind _gridmanagerref_2 (Variables|Default|GetGridManagerRef))
  (bind _pathentry (Variables|Default|GetpathEntry))
  (bind _currentpathindex (Variables|Default|GetcurrentPathIndex))
  (bind _output (Utilities|Array|Get(acopy) _pathentry _currentpathindex))
  (CallFunction|ToggleCellPosition (Variables|Default|GetcurrentGridIndex) false)
  (bind _alpha (Timeline|MoveTimeLine PlayFromStart)
    (:Update
      (Variables|Default|SetisMoving true)
      (Transformation|SetActorLocation (Math|Vector|Lerp(Vector) startPoint newPoint _alpha) false false)
      (bind (_cellexist _cellindex) (Default|GetCellfromWorldSpace _gridmanagerref_2 (Transformation|GetActorLocation)))
      (if _cellexist
        (Variables|Default|SetcurrentGridIndex _cellindex)))
    (:Finished
      (Variables|Default|SetisMoving false)
      (if (!= _gridmanagerref 0)
        (bind (_cellexist_2 _cellindex_2) (Default|GetCellfromWorldSpace _gridmanagerref (Transformation|GetActorLocation)))
        (if _cellexist_2
          (Default|ToggleGridFloor _gridmanagerref_2 false _cellindex_2)
          (Default|ToggleTarget _gridmanagerref_2 (Variables|Default|GetcurrentGridIndex) false)
          (CallFunction|ToggleCellPosition _cellindex_2 true)
          (Math|Integer|IncrementInt (Variables|Default|GetcurrentPathIndex)
            (:%20%20
              (if (< (Variables|Default|GetcurrentPathIndex) (Utilities|Array|Length (Variables|Default|GetpathEntry)))
                (CallFunction|MovetoGridPoint (Math|Vector|MakeVector (.x _output) (.y _output) (.z _returnvalue)) (Math|Vector|MakeVector (.x _returnvalue) (.y _returnvalue) (.z _returnvalue)))))))))))

(event EventBeginPlay
  (bind (_cellexist _cellindex) (Default|GetCellfromWorldSpace (Variables|Default|GetGridManagerRef) (Transformation|GetActorLocation)))
  (if _cellexist
    (bind _output_get (Variables|Default|SetcurrentGridIndex _cellindex))
    (CallFunction|ToggleCellPosition _output_get true)))

(fn ConstructionScript
  (bind _returnvalue (Actor|GetActorOfClass "/Game/Blueprints/Student/Blueprints/Grid/GridManager.GridManager_C"))
  (Variables|Default|SetgridManagerRef _returnvalue))

(fn ToggleCellPosition
  (params (GridCellIndex :type Integer) (hasCharacter :type Boolean))
  (bind _gridmanagerref (Variables|Default|GetGridManagerRef))
  ;[1 1 1] Null ptr check
  (if (!= _gridmanagerref 0)
    (bind _asgrid_floor (Utilities|Casting|CastToGridFloor (Utilities|Array|Get(acopy) (Variables|/Game/Blueprints/Student/Blueprints/Grid/GridManager.GridManager_C|GetGridFloor _gridmanagerref) GridCellIndex)))
    (Default|SetHasCharacter _asgrid_floor hasCharacter)))

(fn SetPath
  (params (pathPoints :type Array%20of%20Vectors))
  (Variables|Default|SetcurrentPathIndex 0)
  (Utilities|Array|Clear (Variables|Default|GetpathEntry))
  (for _array_element pathPoints
    (Utilities|Array|Add (Variables|Default|GetpathEntry) _array_element)))