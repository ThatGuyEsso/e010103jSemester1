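; Base survivor character for a turn-based, grid-based zombie game, selectable while it has actions left.
; It loots adjacent cells, heals wounds with kits and reports inventory to the HUD.
; HUD-driven shoot mode arms free neighbouring cells with one of eight directions, and shots travel along that path.
; A first hit wounds, a zombie hit while wounded kills, and ending an action on an exit cell escapes.
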(event Custom|Select%20Character
  (if (> (Variables|Default|GetcurrentNumberOfActions) 0)
    ;[1 0.419 0.3732] Select Character
    (Rendering|Material|SetMaterial (Variables|Character|GetMesh) 0 (Variables|Material|GetOnMaterial))
    (Variables|CharacterState|SetisSelected true)
    (Default|OnCharacterSelection (Variables|Default|GetGridManagerRef))
    (Default|TogglePlayerButtons (Variables|Component/ObjectRefs|GetHudRef) true)
    (CallFunction|DisplayInventory)))

(event Custom|UnSelect%20Character
  ;[1 0.419 0.3732] Unselect Character
  (Rendering|Material|SetMaterial (Variables|Character|GetMesh) 0 (Variables|Material|GetOffMaterial))
  (Variables|CharacterState|SetisSelected false)
  (Default|TogglePlayerButtons (Variables|Component/ObjectRefs|GetHudRef) false)
  (CallFunction|HideInventory))

(event Custom|OnTurnStart
  ;[1 0.9559 0.4446] Binidng Class
  (CallFunction|ResetActionsLeft))

(event Custom|BindToHUD
  ;[1 1 1] Shoot events
  (EventDispatchers|BindEventtoOnEnterShootMode (Variables|Component/ObjectRefs|GetHudRef) (delegate Custom|EnterShootMode))
  (EventDispatchers|BindEventtoOnExitShootMode (Variables|Component/ObjectRefs|GetHudRef) (delegate Custom|LeaveShootMode)))

(event Custom|LookAtObject
  (params (Target :type Vector%20%28by%20ref%29))
  (bind (_returnvalue _rotationequal) (CallFunction|LookatTargetObject Target))
  (if (not _rotationequal)
    (Variables|Default|SettargetRotate%20Position _returnvalue)
    (bind _alpha (Timeline|TargetRotTimeline PlayFromStart)
      (:Update
        (Transformation|SetActorRotation (Math|Rotator|Lerp(Rotator) (Transformation|GetActorRotation) (Variables|Default|GettargetRotate%20Position) _alpha true))))))

(event Custom|BindToGameManager
  ;[1 0.9559 0.4446] Binidng Class
  (EventDispatchers|BindEventtoEventEndZombieTurn (Variables|Default|GetGameMangerRef) (delegate Custom|OnTurnStart)))

(event Custom|EnterShootMode
  ;[1 1 1] Shoot events
  (if (not (Variables|states|GetinShootMode))
    (CallFunction|InitShootMode)))

(event Custom|LeaveShootMode
  ;[1 1 1] Shoot events
  (if (Variables|states|GetinShootMode)
    (CallFunction|ExitShootMode)))

(event EventDamageSurvivor
  (params (Interface%20Actor :type Actor%20Object%20Reference))
  ;[1 0.6281 0.9937] Damage and death
  (Default|PlaySFX (Variables|Default|GetaudioRef) (Transformation|GetActorLocation) "NewEnumerator0")
  ;;[1 1 1] Checks if player has enough health
  (if (Variables|CharacterState|Getwounded)
    (if (== (Utilities|GetClass Interface%20Actor) "/Game/Blueprints/Student/Blueprints/Characters/BP_BaseZombie.BP_BaseZombie_C")
      (bind _asbp_base_zombie (Utilities|Casting|CastToBP_BaseZombie Interface%20Actor))
      ;;[1 1 1] Interfaces with zombies and game manger
      (Default|SurvivorDeath _asbp_base_zombie self)
      (Default|SurvivorDeath (Variables|Default|GetGameMangerRef) self)
      (Default|DisableCellX (Variables|Default|GetGridManagerRef) (Variables|Default|GetcurrentGridIndex))
      ;;[1 1 1] Spawns emitter
      (Effects|SpawnEmitteratLocation "/Game/Blueprints/Student/Assets/ParticleSystem/BloodSplatter.BloodSplatter" (Transformation|GetActorLocation))
      (Actor|DestroyActor))
    (else
      ;;[1 1 1] If fully healed get wounded
      (Variables|CharacterState|Setwounded true)
      (Effects|SpawnEmitteratLocation "/Game/Blueprints/Student/Assets/ParticleSystem/BloodSplatter.BloodSplatter" (Transformation|GetActorLocation)))))

(event EventGiveLoot
  (params (LootType :type E_Loot%20Enum :default "NewEnumerator0") (Success :type Boolean))
  (if Success
    (Effects|SpawnEmitteratLocation "/Game/Blueprints/Student/Assets/ParticleSystem/StarBurst.StarBurst" (Transformation|GetActorLocation))
    (CallFunction|AddLoot LootType)
    (else
      (Default|ShowPrompt (Variables|Component/ObjectRefs|GetHudRef) "" true))))

(fn ConstructionScript
  (|CallParentFunction))

(fn GetIsSelected
  (return (Variables|CharacterState|GetisSelected)))

(fn EndAction
  (|CallParentFunction)
  (if (<= (Variables|Default|GetcurrentNumberOfActions) 0)
    (CallFunction|UnSelectCharacter))
  (bind _isexit (CallFunction|CheckforExit))
  (if _isexit
    (Effects|SpawnEmitteratLocation "/Game/Blueprints/Student/Assets/ParticleSystem/StarBurst.StarBurst" (Transformation|GetActorLocation))
    (CallFunction|Escape)))

(fn CheckforExit
  (bind _isexit (Default|IsCellXExit (Variables|Default|GetGridManagerRef) (Variables|Default|GetcurrentGridIndex)))
  (return _isexit))

(fn Escape
  (Development|PrintString "escaped" true true "(R=0.486049,G=1.000000,B=0.000000,A=1.000000)")
  (Default|OnPlayerExit (Variables|Default|GetGameMangerRef))
  (Default|PlayUISound (Variables|Default|GetaudioRef) "NewEnumerator2")
  (Actor|DestroyActor))

(fn Init
  (|CallParentFunction)
  (Default|AddSurvivor (Variables|Default|GetGameMangerRef))
  (Variables|Material|SetOffMaterial (Utilities|Array|Get(acopy) (Rendering|Material|GetMaterials (Variables|Character|GetMesh))))
  (CallFunction|BindtoGameManager)
  (bind _asgs_zombie_game (Utilities|Casting|CastToGS_ZombieGame (Game|GetGameState)))
  (Variables|Component/ObjectRefs|SetHudRef (Variables|/Game/Blueprints/Student/GamesModes/GS_ZombieGame.GS_ZombieGame_C|GetHudRef _asgs_zombie_game))
  (CallFunction|BindtoHuD))

(fn LootAdjacentCells
  (bind _asbp_grid_floor (Utilities|Casting|CastToBP_GridFloor (Utilities|Array|Get(acopy) (Variables|/Game/Blueprints/Student/Blueprints/Grid/BP_GridManager.BP_GridManager_C|GetGridFloor (Variables|Default|GetGridManagerRef)) (Variables|Default|GetcurrentGridIndex))))
  (bind _adjacentgridcells (Default|GetAdjacentCellArray _asbp_grid_floor))
  (bind _array_element (Utilities|Array|ForEachLoopwithBreak _adjacentgridcells :!label _label)
    (:LoopBody
      (bind _aboveactor (Default|GetAboveActor _array_element))
      (if (Utilities|DoesObjectImplementInterface _aboveactor "/Game/Blueprints/Student/Blueprints/Interfaces/BPI_Lootable.BPI_Lootable_C")
        (bind _asbp_base_lootable (Utilities|Casting|CastToBP_BaseLootable _aboveactor))
        (Default|Loot _asbp_base_lootable self)
        (CallFunction|LookatObject (Transformation|GetActorLocation _asbp_base_lootable))
        (goto _label Break)))
    (:Completed
      (Development|PrintString "Nothing to loot")
      (CallFunction|UnSelectCharacter))))

(fn AddLoot
  (params (lootType :type E_Loot%20Enum :default "NewEnumerator0"))
  (Utilities|FlowControl|Sequence
    (:then_0
      (switch Utilities|FlowControl|Switch|SwitchonE_Loot lootType
        (:NewEnumerator0
          (CallFunction|GainHealthKit)
          (Default|ShowPrompt (Variables|Component/ObjectRefs|GetHudRef) "Health Kit" false))
        (:NewEnumerator1
          (CallFunction|GainAmmo)
          (Default|ShowPrompt (Variables|Component/ObjectRefs|GetHudRef) "Bullet" false))))
    (:then_1
      (CallFunction|EndAction))))

(fn GainHealthKit
  (bind _result (Math|Integer|IncrementInt (Variables|Inventory|GetcurrHealthKit))
    (:%20%20
      (Development|PrintString (Utilities|String|ToString(Text) (Utilities|Text|FormatText "HealthKits: {kits}" _result))))))

(fn GainAmmo
  (bind _result (Math|Integer|IncrementInt (Variables|inventory|GetcurrAmmo))
    (:%20%20
      (Development|PrintString (Utilities|String|ToString(Text) (Utilities|Text|FormatText "Ammo: {bullets}" _result))))))

(fn UseHealthKit
  (if (> (Variables|Inventory|GetcurrHealthKit) 0)
    (if (Variables|CharacterState|Getwounded)
      (Variables|CharacterState|Setwounded false)
      (Math|Integer|DecrementInt (Variables|Inventory|GetcurrHealthKit)
        (:%20%20
          (bind _asgs_zombie_game (Utilities|Casting|CastToGS_ZombieGame (Game|GetGameState)))
          (Default|SetCurrentKitsAvailable (Variables|/Game/Blueprints/Student/GamesModes/GS_ZombieGame.GS_ZombieGame_C|GetHudRef _asgs_zombie_game) (Variables|Inventory|GetcurrHealthKit))
          (Default|WritePrompt (Variables|/Game/Blueprints/Student/GamesModes/GS_ZombieGame.GS_ZombieGame_C|GetHudRef _asgs_zombie_game) "Fully Healed")))
      (else
        (bind _asgs_zombie_game_2 (Utilities|Casting|CastToGS_ZombieGame (Game|GetGameState)))
        (Default|WritePrompt (Variables|/Game/Blueprints/Student/GamesModes/GS_ZombieGame.GS_ZombieGame_C|GetHudRef _asgs_zombie_game_2) "Survivor Is not wounded")))
    (else
      (bind _asgs_zombie_game_3 (Utilities|Casting|CastToGS_ZombieGame (Game|GetGameState)))
      (Default|WritePrompt (Variables|/Game/Blueprints/Student/GamesModes/GS_ZombieGame.GS_ZombieGame_C|GetHudRef _asgs_zombie_game_3) "Survivor Has No Health Kits"))))

(fn DisplayInventory
  (if (> (Variables|Inventory|GetcurrHealthKit) 0)
    (bind _asgs_zombie_game (Utilities|Casting|CastToGS_ZombieGame (Game|GetGameState)))
    (Default|ToggleHealthKit (Variables|/Game/Blueprints/Student/GamesModes/GS_ZombieGame.GS_ZombieGame_C|GetHudRef _asgs_zombie_game) true)
    (Default|SetCurrentKitsAvailable (Variables|/Game/Blueprints/Student/GamesModes/GS_ZombieGame.GS_ZombieGame_C|GetHudRef _asgs_zombie_game) (Variables|Inventory|GetcurrHealthKit))
    (if (> (Variables|inventory|GetcurrAmmo) 0)
      (Default|ToggleBullets (Variables|/Game/Blueprints/Student/GamesModes/GS_ZombieGame.GS_ZombieGame_C|GetHudRef _asgs_zombie_game) true)
      (Default|SetCurrentBulletsAvailable (Variables|/Game/Blueprints/Student/GamesModes/GS_ZombieGame.GS_ZombieGame_C|GetHudRef _asgs_zombie_game) (Variables|inventory|GetcurrAmmo)))
    (elif (> (Variables|inventory|GetcurrAmmo) 0)
      (bind _asgs_zombie_game_2 (Utilities|Casting|CastToGS_ZombieGame (Game|GetGameState)))
      (Default|ToggleBullets (Variables|/Game/Blueprints/Student/GamesModes/GS_ZombieGame.GS_ZombieGame_C|GetHudRef _asgs_zombie_game_2) true)
      (Default|SetCurrentBulletsAvailable (Variables|/Game/Blueprints/Student/GamesModes/GS_ZombieGame.GS_ZombieGame_C|GetHudRef _asgs_zombie_game_2) (Variables|inventory|GetcurrAmmo)))))

(fn HideInventory
  (bind _asgs_zombie_game (Utilities|Casting|CastToGS_ZombieGame (Game|GetGameState)))
  (Default|ToggleHealthKit (Variables|/Game/Blueprints/Student/GamesModes/GS_ZombieGame.GS_ZombieGame_C|GetHudRef _asgs_zombie_game) false)
  (Default|ToggleBullets (Variables|/Game/Blueprints/Student/GamesModes/GS_ZombieGame.GS_ZombieGame_C|GetHudRef _asgs_zombie_game) false))

(fn HasActions
  (return (> (Variables|Default|GetcurrentNumberOfActions) 0)))

(fn InitShootMode
  (if (> (Variables|inventory|GetcurrAmmo) 0)
    (bind _asbp_grid_floor (Utilities|Casting|CastToBP_GridFloor (Utilities|Array|Get(acopy) (Variables|/Game/Blueprints/Student/Blueprints/Grid/BP_GridManager.BP_GridManager_C|GetGridFloor (Variables|Default|GetGridManagerRef)) (Variables|Default|GetcurrentGridIndex))))
    (bind _cellcoordinate (Default|GetGridCoordinate _asbp_grid_floor))
    (LocalVariables|SetSurvivorCoord _cellcoordinate)
    (bind _adjacentgridcells (Default|GetAdjacentCellArray _asbp_grid_floor))
    (for _array_element _adjacentgridcells
      (bind _isfree (Default|IsCellFree _array_element))
      (if _isfree
        (bind _cellcoordinate_2 (Default|GetGridCoordinate _array_element))
        (bind _alarmdir (CallFunction|ResolveRelativeDirections _cellcoordinate_2 (LocalVariables|GetSurvivorCoord)))
        (Default|SetUpShootTrigger _array_element _alarmdir)))
    (Variables|states|SetinShootMode true)))

(fn ExitShootMode
  (bind _asbp_grid_floor (Utilities|Casting|CastToBP_GridFloor (Utilities|Array|Get(acopy) (Variables|/Game/Blueprints/Student/Blueprints/Grid/BP_GridManager.BP_GridManager_C|GetGridFloor (Variables|Default|GetGridManagerRef)) (Variables|Default|GetcurrentGridIndex))))
  (bind _adjacentgridcells (Default|GetAdjacentCellArray _asbp_grid_floor))
  (for _array_element _adjacentgridcells
    (Default|Deactivate _array_element))
  (Variables|states|SetinShootMode false))

(fn Shoot
  (params (shootCell :type Int%202D%20Structure))
  (bind _asbp_grid_floor (Default|GetCellfromCoordinate (Variables|Default|GetGridManagerRef) shootCell))
  (Default|ShootAlongPath _asbp_grid_floor)
  (Math|Integer|DecrementInt (Variables|Default|GetcurrentNumberOfActions)
    (:%20%20
      (bind _result (Math|Integer|DecrementInt (Variables|inventory|GetcurrAmmo))
        (:%20%20
          (Default|SetCurrentBulletsAvailable (Variables|Component/ObjectRefs|GetHudRef) _result)
          (CallFunction|ExitShootMode))))))

(fn ResolveRelativeDirections
  (params (adjacentCellCoord :type Int%202D%20Structure) (surivivorCoordinate :type Int%202D%20Structure))
  (LocalVariables|SetoriginalCoord surivivorCoordinate)
  (LocalVariables|SetcurrCellCoord adjacentCellCoord)
  (if (and (== (.x (LocalVariables|GetoriginalCoord)) (.x (LocalVariables|GetcurrCellCoord))) (< (.y (LocalVariables|GetoriginalCoord)) (.y (LocalVariables|GetcurrCellCoord))))
    (return "NewEnumerator0")
    (elif (and (== (.x (LocalVariables|GetoriginalCoord)) (.x (LocalVariables|GetcurrCellCoord))) (> (.y (LocalVariables|GetoriginalCoord)) (.y (LocalVariables|GetcurrCellCoord))))
      (return "NewEnumerator1")
      (elif (and (> (.x (LocalVariables|GetoriginalCoord)) (.x (LocalVariables|GetcurrCellCoord))) (== (.y (LocalVariables|GetoriginalCoord)) (.y (LocalVariables|GetcurrCellCoord))))
        (return "NewEnumerator3")
        (elif (and (< (.x (LocalVariables|GetoriginalCoord)) (.x (LocalVariables|GetcurrCellCoord))) (== (.y (LocalVariables|GetoriginalCoord)) (.y (LocalVariables|GetcurrCellCoord))))
          (return "NewEnumerator2")
          (elif (and (> (.x (LocalVariables|GetoriginalCoord)) (.x (LocalVariables|GetcurrCellCoord))) (< (.y (LocalVariables|GetoriginalCoord)) (.y (LocalVariables|GetcurrCellCoord))))
            (return "NewEnumerator4")
            (elif (and (< (.x (LocalVariables|GetoriginalCoord)) (.x (LocalVariables|GetcurrCellCoord))) (< (.y (LocalVariables|GetoriginalCoord)) (.y (LocalVariables|GetcurrCellCoord))))
              (return "NewEnumerator5")
              (elif (and (> (.x (LocalVariables|GetoriginalCoord)) (.x (LocalVariables|GetcurrCellCoord))) (> (.y (LocalVariables|GetoriginalCoord)) (.y (LocalVariables|GetcurrCellCoord))))
                (return "NewEnumerator7")
                (elif (and (< (.x (LocalVariables|GetoriginalCoord)) (.x (LocalVariables|GetcurrCellCoord))) (> (.y (LocalVariables|GetoriginalCoord)) (.y (LocalVariables|GetcurrCellCoord))))
                  (return "NewEnumerator6"))))))))))