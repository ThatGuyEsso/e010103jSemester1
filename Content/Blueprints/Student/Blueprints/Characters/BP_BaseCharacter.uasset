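; Base character for a turn-based grid game that walks cell paths and spends limited actions per turn.
; MoveToGridPoint turns toward the next point, then lerps there on timelines, recursing through the path while updating grid floor occupancy.
; Finishing a path costs an action; at zero it asks GameManager to resolve turns and refills.
; Walking is faked by swapping static meshes once per path step.
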(event Custom|MoveToGridPoint
  (params (newPoint :type Vector) (startPoint :type Vector))
  (bind _returnvalue (Transformation|GetActorLocation))
  (bind _pathentry (Variables|Pathing|GetpathEntry))
  (bind _gridmanagerref (Variables|Component/ObjectRefs|GetGridManagerRef))
  (bind _gridmanagerref_2 (Variables|Component/ObjectRefs|GetGridManagerRef))
  (bind _currentpathindex (Variables|Pathing|GetcurrentPathIndex))
  (bind _output (Utilities|Array|Get(acopy) _pathentry _currentpathindex))
  ;[1 1 1] Quick check if character has the actions to allow this to be performed
  (bind _canperform (CallFunction|GetCanPerformAction))
  (if _canperform
    ;[1 1 1] Get rotation point
    (bind (_returnvalue_2 _rotationequal) (CallFunction|LookatTargetPoint))
    (if _rotationequal
      ;[0.9581 1 0] Move to point on grid event
      ;;[1 1 1] Disable and remove themselve from current grid position. A grid can only have one character
      (CallFunction|SetCurrentGridAboveActor false (Variables|Pathing|GetcurrentGridIndex) :!label _label)
      (CallFunction|ToggleCellPosition (Variables|Pathing|GetcurrentGridIndex) false)
      (CallFunction|StartWalkAnim)
      ;;[1 1 1] Start lerping from start each time to keep consisten speed
      (bind _alpha (Timeline|MoveTimeLine PlayFromStart)
        (:Update
          ;;[1 1 1] Lerp between current position and target
          ;;;[1 1 1] While updating player is definitely moving
          (Variables|CharacterState|SetisMoving true)
          (Transformation|SetActorLocation (Math|Vector|Lerp(Vector) startPoint newPoint _alpha) false false)
          (bind (_cellexist _cellindex) (Default|GetCellfromWorldSpace _gridmanagerref_2 (Transformation|GetActorLocation)))
          (if _cellexist
            (Variables|Pathing|SetcurrentGridIndex _cellindex)))
        (:Finished
          ;;[1 1 1] On Finished check if Gridmanager isn't null
          (if (!= _gridmanagerref 0)
            ;;;[1 1 1] Get current cell character is on
            (bind (_cellexist_2 _cellindex_2) (Default|GetCellfromWorldSpace _gridmanagerref (Transformation|GetActorLocation)))
            ;;[1 1 1] If cell exist
            (if _cellexist_2
              ;;[1 1 1] Turn cell off, and incase it is the target make it not the target then update the cell to show it is currently holding a character
              (Default|ToggleGridFloor _gridmanagerref_2 false _cellindex_2)
              (Default|ToggleTarget _gridmanagerref_2 (Variables|Pathing|GetcurrentGridIndex) false)
              (CallFunction|ToggleCellPosition _cellindex_2 true)
              ;;[1 1 1] Increment path index
              (Math|Integer|IncrementInt (Variables|Pathing|GetcurrentPathIndex)
                (:%20%20
                  (if (< (Variables|Pathing|GetcurrentPathIndex) (Utilities|Array|Length (Variables|Pathing|GetpathEntry)))
                    ;;[1 1 1] In this case the next position is equal to the new path index, so target location is the next point in array, and current point is actors location
                    (CallFunction|MovetoGridPoint (Math|Vector|MakeVector (.x _output) (.y _output) (.z _returnvalue)) (Math|Vector|MakeVector (.x _returnvalue) (.y _returnvalue) (.z _returnvalue)))
                    (CallFunction|UpdateWalkFrame)
                    (else
                      ;;[1 1 1] In that case stop character
                      ;;;[1 1 1] Destination reached so stop moving
                      (Variables|CharacterState|SetisMoving false)
                      ;;;[1 1 1] Clear old path
                      (CallFunction|ClearCurrentPath)
                      ;;;[1 1 1] One action has been completed so end it
                      (CallFunction|EndAction)
                      ;;;[1 1 1] above actor equal this
                      (CallFunction|SetCurrentGridAboveActor true (Variables|Pathing|GetcurrentGridIndex))
                      (CallFunction|UpdateWalkFrame)))))))))
      (else
        (Variables|Default|SettargetRotate%20Position _returnvalue_2)
        ;[1 1 1] Rotate actor to face point
        (bind _alpha_2 (Timeline|RotateTimeLine PlayFromStart)
          (:Update
            (Transformation|SetActorRotation (Math|Rotator|Lerp(Rotator) (Transformation|GetActorRotation) (Variables|Default|GettargetRotate%20Position) _alpha_2 true)))
          (:Finished
            (goto _label)))))))

(event EventBeginPlay
  ;[0.9581 1 0] Move to point on grid event
  (CallFunction|Init))

(fn ConstructionScript
  (bind _returnvalue (Actor|GetActorOfClass "/Game/Blueprints/Student/Blueprints/Grid/BP_GridManager.BP_GridManager_C"))
  (Variables|Default|SetgridManagerRef _returnvalue)
  (bind _returnvalue_2 (Actor|GetActorOfClass "/Game/Blueprints/Student/Blueprints/GameManagement/GameManager.GameManager_C"))
  (Variables|Component/ObjectRefs|SetGameMangerRef _returnvalue_2)
  (bind _returnvalue_3 (Actor|GetActorOfClass "/Game/Blueprints/Student/Blueprints/GameManagement/AudioManager.AudioManager_C"))
  (Variables|Default|SetaudioRef _returnvalue_3))

(fn ToggleCellPosition
  (params (GridCellIndex :type Integer) (hasCharacter :type Boolean))
  (bind _gridmanagerref (Variables|Component/ObjectRefs|GetGridManagerRef))
  ;[1 1 1] Null ptr check
  (if (!= _gridmanagerref 0)
    (bind _asbp_grid_floor (Utilities|Casting|CastToBP_GridFloor (Utilities|Array|Get(acopy) (Variables|/Game/Blueprints/Student/Blueprints/Grid/BP_GridManager.BP_GridManager_C|GetGridFloor _gridmanagerref) GridCellIndex)))
    (Default|SetHasCharacter _asbp_grid_floor hasCharacter)))

(fn SetPath
  (params (pathPoints :type Array%20of%20Vectors))
  (Variables|Pathing|SetcurrentPathIndex 0)
  (Utilities|Array|Clear (Variables|Pathing|GetpathEntry))
  (for _array_element pathPoints
    (Utilities|Array|Add (Variables|Pathing|GetpathEntry) _array_element)))

(fn Init
  (bind (_cellexist _cellindex) (Default|GetCellfromWorldSpace (Variables|Component/ObjectRefs|GetGridManagerRef) (Transformation|GetActorLocation)))
  (if _cellexist
    (bind _output_get (Variables|Pathing|SetcurrentGridIndex _cellindex))
    (CallFunction|SetCurrentGridAboveActor true _output_get)
    (CallFunction|ToggleCellPosition _output_get true)
    (Variables|settings|SetcurrentNumberOfActions (Variables|settings|GetmaxNumberOfActions))))

(fn EndAction
  ;[1 1 1] If character has no actions left character needs to tell game manager that their individual turn has ended(Note other character on it team might still have more turns left)
  (Math|Integer|DecrementInt (Variables|settings|GetcurrentNumberOfActions)
    (:%20%20
      (if (not (> (Variables|settings|GetcurrentNumberOfActions) 0))
        (Default|ResolvePlayerTurns (Variables|Component/ObjectRefs|GetGameMangerRef))
        (Variables|settings|SetcurrentNumberOfActions (Variables|settings|GetmaxNumberOfActions))))))

(fn ClearCurrentPath
  (Utilities|Array|Clear (Variables|Pathing|GetpathEntry)))

(fn GetCanPerformAction
  (if (> (Variables|settings|GetcurrentNumberOfActions) 0)
    (return true)
    (else
      (return false))))

(fn ResetActionsLeft
  (Variables|settings|SetcurrentNumberOfActions (Variables|settings|GetmaxNumberOfActions)))

(fn GetMaxSteps
  (return (Variables|CharacterActions|GetmaxSteps)))

(fn LookatTargetPoint
  (bind _returnvalue (Transformation|GetActorLocation))
  (bind _returnvalue_2 (Transformation|GetActorRotation))
  (bind _pathentry (Variables|Pathing|GetpathEntry))
  (bind _currentpathindex (Variables|Pathing|GetcurrentPathIndex))
  (bind _output (Utilities|Array|Get(acopy) _pathentry _currentpathindex))
  (bind _returnvalue_3 (Math|Rotator|FindLookatRotation _returnvalue _output))
  (bind _returnvalue_4 (Math|Rotator|MakeRotator (.roll _returnvalue_2) (.pitch _returnvalue_2) (.yaw _returnvalue_3)))
  (return _returnvalue_4 (Math|Rotator|Equal(Rotator) (Transformation|GetActorRotation) _returnvalue_4 0.0001)))

(fn LookatTargetObject
  (params (Target :type Vector%20%28by%20ref%29))
  (bind _returnvalue (Transformation|GetActorLocation))
  (bind _returnvalue_2 (Transformation|GetActorRotation))
  (bind _returnvalue_3 (Math|Rotator|FindLookatRotation _returnvalue Target))
  (bind _returnvalue_4 (Math|Rotator|MakeRotator (.roll _returnvalue_2) (.pitch _returnvalue_2) (.yaw _returnvalue_3)))
  (return _returnvalue_4 (Math|Rotator|Equal(Rotator) (Transformation|GetActorRotation) _returnvalue_4 0.0001)))

(fn SetCurrentGridAboveActor
  (params (cellHasActor :type Boolean) (cell%20Index :type Integer))
  (bind _gridmanagerref (Variables|Component/ObjectRefs|GetGridManagerRef))
  ;[1 1 1] Null ptr check
  (if (!= _gridmanagerref 0)
    (bind _asbp_grid_floor (Utilities|Casting|CastToBP_GridFloor (Utilities|Array|Get(acopy) (Variables|/Game/Blueprints/Student/Blueprints/Grid/BP_GridManager.BP_GridManager_C|GetGridFloor _gridmanagerref) cell%20Index)))
    (if cellHasActor
      (Default|SetAboveActor _asbp_grid_floor self)
      (else
        (Default|SetAboveActor _asbp_grid_floor)))))

(fn UpdateWalkFrame
  (bind _walkframes (Variables|Animation|GetWalkFrames))
  (bind _returnvalue (Utilities|Array|Length _walkframes))
  (if (Variables|CharacterState|GetisMoving)
    (if (> _returnvalue 0)
      (Math|Integer|IncrementInt (Variables|Animation|GetanimIndex)
        (:%20%20
          (if (>= (Variables|Animation|GetanimIndex) _returnvalue)
            (bind _output_get (Variables|Animation|SetanimIndex 0))
            (Components|StaticMesh|SetStaticMesh (Variables|Default|GetMesh) (Utilities|Array|Get(acopy) (Variables|Animation|GetWalkFrames) _output_get))
            (else
              (Components|StaticMesh|SetStaticMesh (Variables|Default|GetMesh) (Utilities|Array|Get(acopy) (Variables|Animation|GetWalkFrames) (Variables|Animation|GetanimIndex)))))))
      (else
        (Components|StaticMesh|SetStaticMesh (Variables|Default|GetMesh) (Variables|Animation|GetIdleFrame) :!label _label)))
    (else
      (goto _label))))

(fn StartWalkAnim
  (if (> (Utilities|Array|Length (Variables|Animation|GetWalkFrames)) 0)
    (Components|StaticMesh|SetStaticMesh (Variables|Default|GetMesh) (Utilities|Array|Get(acopy) (Variables|Animation|GetWalkFrames) (Variables|Animation|GetanimIndex)))))