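; Base zombie character for a turn-based grid game, wandering, chasing and attacking survivors with a limited number of actions per turn.
; A macro-switched state machine checks adjacent cells for attack targets and uses a forward box trace to spot survivors to chase.
; It sends chase or recursively retried random wander cells to the grid manager, while attacks turn it with a timeline and damage the survivor.
; EndAction repeats the turn until actions run out, then notifies the game manager.
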(event Custom|FaceTarget
  (params (Target :type Vector%20%28by%20ref%29))
  ;[1 1 1] Get rotation point
  (bind (_returnvalue _rotationequal) (CallFunction|LookatTargetObject Target))
  (if (not _rotationequal)
    (Variables|Default|SettargetRotate%20Position _returnvalue)
    ;[1 1 1] Rotate to look at target
    (bind _alpha (Timeline|RotationToTargetTime PlayFromStart)
      (:Update
        (Transformation|SetActorRotation (Math|Rotator|Lerp(Rotator) (Transformation|GetActorRotation) (Variables|Default|GettargetRotate%20Position) _alpha true))))))

(event Custom|ZombieTake%20Turn
  (bind _survivortarget (Variables|Component/ObjectRefs|GetSurvivorTarget))
  ;[1 1 1] Turn handling
  (if (not (Variables|Default|GetgameEnded))
    (CallFunction|GetSurvivorsinRange)
    (Utilities|SwitchState
      (:Wander
        (if (Variables|CharacterState|GethasTarget)
          (Utilities|SwitchCurrentTargetType :!label _label
            (:Survivor
              (bind (_array_index _cellexist) (CallFunction|GetLocationOfTargetSurvivor :!label _label_2))
              (if _cellexist
                (Default|ZombieFoundMoveLocation (Variables|Default|GetGridManagerRef) self _array_index))))
          (else
            (bind _output_get (CallFunction|CheckifPlayerIsinVision))
            (if _output_get
              (CallFunction|SetZombieState "NewEnumerator1")
              (goto _label_2)
              (else
                (bind _cellindex (CallFunction|GetRandomPositionAroundCharacter (Variables|Settings|GetwanderRange)))
                (Default|ZombieFoundMoveLocation (Variables|Default|GetGridManagerRef) self _cellindex))))))
      (:Chase
        (goto _label))
      (:Attack
        (CallFunction|FaceTarget (Transformation|GetActorLocation _survivortarget))
        (Default|DamageSurvivor _survivortarget self)
        (CallFunction|EndAction)))))

(event Custom|OnTurnStart
  ;[1 1 1] Bwgin plAY
  (CallFunction|ResetActionsLeft))

(event EventSurvivorDeath
  (params (Interface%20Actor :type Actor%20Object%20Reference))
  ;[1 1 1] Event target survivor died
  (Utilities|FlowControl|Delay 0.2)
  (Variables|Component/ObjectRefs|SetSurvivorTarget 0)
  (CallFunction|SetZombieState "NewEnumerator0")
  (Variables|CharacterState|SethasTarget false))

(event EventEndGame
  (Variables|Default|SetgameEnded true))

(event EventStartGame
  (params (Interface%20Actor :type Actor%20Object%20Reference))
  (CallFunction|Init))

(event EventZombieMoveLocationIsNotValid
  ;[1 1 1] Interface events (Zombie Actions)
  (CallFunction|ZombieTakeTurn))

(event EventBeginPlay
  ;[1 1 1] Bwgin plAY
  (EventDispatchers|BindEventtoEventEndPlayerTurn (Variables|Default|GetGameMangerRef) (delegate Custom|OnTurnStart)))

(fn ConstructionScript
  (|CallParentFunction))

(fn GetRandomPositionAroundCharacter
  (params (moveRange :type Integer))
  (LocalVariables|SetstepDistance moveRange)
  (bind _asbp_grid_floor (Utilities|Casting|CastToBP_GridFloor (Utilities|Array|Get(acopy) (Variables|/Game/Blueprints/Student/Blueprints/Grid/BP_GridManager.BP_GridManager_C|GetGridFloor (Variables|Default|GetGridManagerRef)) (Variables|Default|GetcurrentGridIndex))))
  (bind _cellcoordinate (Default|GetGridCoordinate _asbp_grid_floor))
  (bind _output_get (LocalVariables|SetcurrentCellCoordinate _cellcoordinate))
  (bind _output_get_2 (LocalVariables|SetnewCellCoordinate (Utilities|Struct|MakeInt2D (+ (.x _output_get) (Math|Random|RandomIntegerinRange (* (LocalVariables|GetstepDistance) -1) (LocalVariables|GetstepDistance))) (+ (Math|Random|RandomIntegerinRange (* (LocalVariables|GetstepDistance) -1) (LocalVariables|GetstepDistance)) (.y _output_get)))))
  (bind (_asbp_grid_floor_2 _isvalid _array_index) (Default|GetCellfromCoordinate (Variables|Default|GetGridManagerRef) _output_get_2))
  (if _isvalid
    (bind _isobstructed (Default|GetIsObstructed _asbp_grid_floor_2))
    (if _isobstructed
      _
      (else
        (return _array_index))))
  (CallFunction|GetRandomPositionAroundCharacter (Variables|Settings|GetwanderRange)))

(fn EndAction
  ;[1 1 1] If character has no actions left character needs to tell game manager that their individual turn has ended(Note other character on it team might still have more turns left)
  (Math|Integer|DecrementInt (Variables|Default|GetcurrentNumberOfActions)
    (:%20%20
      (if (> (Variables|Default|GetcurrentNumberOfActions) 0)
        (CallFunction|ZombieTakeTurn)
        (else
          (Default|ResolveZombieTurns (Variables|Default|GetGameMangerRef))
          (Variables|Default|SetcurrentNumberOfActions (Variables|Default|GetmaxNumberOfActions)))))))

(fn CheckifPlayerIsinVision
  (bind _visionpoint (Variables|Default|GetVisionPoint))
  (bind _visionwidth (Variables|Settings|GetvisionWidth))
  (bind _returnvalue (Transformation|GetWorldLocation _visionpoint))
  (bind _outhit (Collision|BoxTraceByChannel _returnvalue (+ _returnvalue (* (Math|Vector|GetForwardVector _visionpoint) (Variables|Settings|GetvisionRange))) (Math|Vector|MakeVector _visionwidth _visionwidth 4e+01) "0, 0, 0" "TraceTypeQuery1" false 0 "None"))
  (if (== (Utilities|GetClass (.HitActor (Collision|BreakHitResult _outhit))) "/Game/Blueprints/Student/Blueprints/Characters/BP_BaseSurvivor.BP_BaseSurvivor_C")
    (bind _asbp_base_survivor (Utilities|Casting|CastToBP_BaseSurvivor (.HitActor (Collision|BreakHitResult _outhit))))
    (Variables|Component/ObjectRefs|SetSurvivorTarget _asbp_base_survivor)
    (bind _output_get (Variables|CharacterState|SethasTarget true))
    (Variables|CharacterState|SetcurrentTargetType "NewEnumerator0")
    (return _output_get)
    (else
      (return false))))

(fn GetLocationOfTargetSurvivor
  (bind (_array_index _cellexist) (Default|GetCellwithCharacter (Variables|Default|GetGridManagerRef) (Variables|Component/ObjectRefs|GetSurvivorTarget)))
  (if _cellexist
    (bind _asbp_grid_floor (Utilities|Casting|CastToBP_GridFloor (Utilities|Array|Get(acopy) (Variables|/Game/Blueprints/Student/Blueprints/Grid/BP_GridManager.BP_GridManager_C|GetGridFloor (Variables|Default|GetGridManagerRef)) _array_index)))
    (bind _output (Default|GetClosesCelltoPoint _asbp_grid_floor (Transformation|GetActorLocation)))
    (bind (_cellexist_2 _cellindex) (Default|GetCellfromWorldSpace (Variables|Default|GetGridManagerRef) (Transformation|GetActorLocation _output)))
    (if _cellexist_2
      (return _cellindex true)
      (else
        (return 0 false)))))

(fn SetZombieState
  (params (newState :type BaseZombieStates%20Enum :default "NewEnumerator0"))
  (Variables|CharacterState|SetcurrentState newState))

(fn SetCurrentTargetType
  (params (newTargetType :type ZombieTargetType%20Enum :default "NewEnumerator2"))
  (Variables|CharacterState|SetcurrentTargetType newTargetType))

(fn GetSurvivorsinRange
  (bind _asbp_grid_floor (Utilities|Casting|CastToBP_GridFloor (Utilities|Array|Get(acopy) (Variables|/Game/Blueprints/Student/Blueprints/Grid/BP_GridManager.BP_GridManager_C|GetGridFloor (Variables|Default|GetGridManagerRef)) (Variables|Default|GetcurrentGridIndex))))
  (bind _adjacentgridcells (Default|GetAdjacentCellArray _asbp_grid_floor))
  (for _array_element _adjacentgridcells
    (bind _aboveactor (Default|GetAboveActor _array_element))
    (if (!= _aboveactor 0)
      (bind _hascharacter (Default|GetHasCharacter _array_element))
      (if _hascharacter
        (if (Actor|ActorHasTag _aboveactor "Survivor")
          (bind _asbp_base_survivor (Utilities|Casting|CastToBP_BaseSurvivor _aboveactor)
            (:then
              (Variables|Component/ObjectRefs|SetSurvivorTarget _asbp_base_survivor)
              (CallFunction|SetZombieState "NewEnumerator2")
              (Variables|CharacterState|SethasTarget true)
              (return))
            (:CastFailed
              (Development|PrintString "failed to print to a survivor")))
          (else
            ;[1 1 1] Incase player is no longer in range or never was, chase or wander
            (Utilities|SwitchState :!label _label
              (:Wander
                (CallFunction|SetZombieState "NewEnumerator0"))
              (:Chase
                (CallFunction|SetZombieState "NewEnumerator1" :!label _label_2))
              (:Attack
                (goto _label_2)))))
        (else
          (goto _label)))
      (else
        (goto _label)))))