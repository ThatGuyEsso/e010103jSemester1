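; Game manager for a turn-based survivors-versus-zombies grid level, handling spawning, turns, HUD and win or loss.
; BeginPlay spawns survivors and a zombie at random GridManager positions, then creates the HUD.
; Turn counters flip between Player and Zombie turns, with zombies acting sequentially by index and MoveCharacter passing grid paths to the active character.
; Survivor deaths and exits feed ResolveGame: any escape wins and allows early escape, none remaining otherwise loses.
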(event Custom|spawnZombie
  ;[0.3182 0.3856 1] Spawn Zombie
  (bind _position (Default|GetRandomPositiononGrid (Variables|Component/ObjectReferences|GetgridManagerRef)))
  (bind _returnvalue (Game|SpawnActorfromClass "/Game/Blueprints/Student/Blueprints/Characters/BP_BaseZombie.BP_BaseZombie_C" (Math|Transform|MakeTransform (+ _position (Variables|Settings|GetspawnOffSet))) "Undefined" 0 0))
  (Utilities|Array|Add (Variables|Characters|GetzombieRef) _returnvalue))

(event Custom|SetUpHUDUI
  ;[0 1 0.03596] HUD Update
  (bind _returnvalue (UserInterface|CreateWidget "/Game/Blueprints/Student/Blueprints/UI/HUD.HUD_C"))
  (bind _output_get (Variables|Component/ObjectReferences|SetHudRef _returnvalue))
  (UserInterface|Viewport|AddtoViewport _output_get 0)
  (CallFunction|StartGame))

(event Custom|End%20Zombie%20Turn
  ;[0.6095 0.6147 1] End Zombie turn
  (Variables|GameStates|SetcurrentTurn "NewEnumerator0")
  (CallFunction|ResolveTurnLabels)
  (Variables|TurnData|SetnumSurvivorTurnsLeft (Variables|TurnData|GetnumberOfSurvivors))
  (Default|CallEventEndZombieTurn))

(event Custom|End%20Player%20Turn
  ;[0.5406 0.5633 1] Set Active survior role to null and set current turn to zombie turn
  (if (!= (Variables|Component/ObjectReferences|GetActiveSurvivorRef) 0)
    (Default|UnSelectCharacter (Variables|Component/ObjectReferences|GetActiveSurvivorRef))
    (Variables|Component/ObjectReferences|SetActiveSurvivorRef 0)
    (Variables|GameStates|SetcurrentTurn "NewEnumerator1")
    (else
      (Variables|Component/ObjectReferences|SetActiveSurvivorRef 0)
      (Variables|GameStates|SetcurrentTurn "NewEnumerator1")))
  (CallFunction|ResolveTurnLabels)
  (Default|CallEventEndPlayerTurn)
  (CallFunction|StartAIActions))

(event Custom|OnSpawnPlayer
  ;[0.3182 0.3856 1] Spawn Player
  (bind _position (Default|GetRandomPositiononGrid (Variables|Component/ObjectReferences|GetgridManagerRef)))
  (Game|SpawnActorfromClass "/Game/Blueprints/Student/Blueprints/Characters/BP_BaseSurvivor.BP_BaseSurvivor_C" (Math|Transform|MakeTransform (+ _position (Variables|Settings|GetspawnOffSet))) "Undefined" 0 0))

(event EventMoveZombietoGridPoint
  (CallFunction|MoveCharacter))

(event EventSurvivorDeath
  (params (Interface%20Actor :type Actor%20Object%20Reference))
  ;[1 1 1] Survivors Left decrement
  (Math|Integer|DecrementInt (Variables|TurnData|GetcurrentNumberOfSurvivors)
    (:%20%20
      ;[1 1 1] Determines wether survivor dies or not
      (CallFunction|ResolveGame))))

(event EventOnPlayerExit
  (Math|Integer|IncrementInt (Variables|Win/LossCondition|GetsurvivorsEscaped)
    (:%20%20
      (Math|Integer|DecrementInt (Variables|TurnData|GetcurrentNumberOfSurvivors)
        (:%20%20
          (CallFunction|ResolveGame))))))

(event EventBeginPlay
  ;[0 1 0.07877] Begin Play
  (Utilities|FlowControl|Sequence
    (:then_0
      (Utilities|FlowControl|Delay 0.0)
      (while (< (Variables|TurnData|GetcurrentNumberOfSurvivors) (Variables|TurnData|GetnumberOfSurvivors))
        (CallFunction|OnSpawnPlayer)
        (bind _result (Math|Integer|IncrementInt (Variables|TurnData|GetcurrentNumberOfSurvivors))
          (:%20%20
            (Development|PrintString (Utilities|String|ToString(Integer) _result)))))
      (CallFunction|SpawnZombie)
      (bind _output_get (Variables|TurnData|SetcurrentNumberOfSurvivors (Variables|TurnData|GetnumberOfSurvivors)))
      (Variables|TurnData|SetnumSurvivorTurnsLeft _output_get)
      (Variables|TurnData|SetnumZombieTurnsLeft (Utilities|Array|Length (Variables|Characters|GetzombieRef))))
    (:then_1
      (CallFunction|SetUpHUDUI))
    (:then_2
      (Game|SetGamePaused false))))

(fn ConstructionScript
  (bind _returnvalue (Actor|GetActorOfClass "/Game/Blueprints/Student/Blueprints/Grid/GridManager.GridManager_C"))
  (Variables|Component/ObjectReferences|SetgridManagerRef _returnvalue))

(fn MoveCharacter
  (bind _activesurvivorref (Variables|Component/ObjectReferences|GetActiveSurvivorRef))
  (bind _gridmanagerref (Variables|Component/ObjectReferences|GetgridManagerRef))
  (bind _activesurvivorref_2 (Variables|Component/ObjectReferences|GetActiveSurvivorRef))
  (bind _zombieref (Variables|Characters|GetzombieRef))
  (bind _currentactivezombieindex (Variables|TurnData|GetcurrentActiveZombieIndex))
  (bind _returnvalue (Transformation|GetActorLocation _activesurvivorref))
  (bind _output (Utilities|Array|Get(acopy) _zombieref _currentactivezombieindex))
  (bind _returnvalue_2 (Transformation|GetActorLocation _output))
  (switch Utilities|FlowControl|Switch|SwitchonTurnState (Variables|GameStates|GetcurrentTurn)
    (:NewEnumerator0
      (if (Variables|TurnData|GetcanCharacterMove)
        (if (!= (Variables|Component/ObjectReferences|GetActiveSurvivorRef) 0)
          (if (not (Variables|/Game/Blueprints/Student/Blueprints/Characters/BP_BaseCharacter.BP_BaseCharacter_C|GetisMoving _activesurvivorref_2))
            (if (!= _gridmanagerref 0)
              ;[1 1 1] Passes defined path to character. First Point character position last target
              (bind _pathpositions (Default|GetCurrentPath _gridmanagerref))
              (Default|SetPath _activesurvivorref_2 _pathpositions)
              (Default|MovetoGridPoint _activesurvivorref (Math|Vector|MakeVector (.x (Utilities|Array|Get(acopy) _pathpositions)) (.y (Utilities|Array|Get(acopy) _pathpositions)) (.z _returnvalue)) (Math|Vector|MakeVector (.x _returnvalue) (.y _returnvalue) (.z _returnvalue))))))))
    (:NewEnumerator1
      (if (not (Variables|/Game/Blueprints/Student/Blueprints/Characters/BP_BaseCharacter.BP_BaseCharacter_C|GetisMoving _output))
        (if (!= (Variables|Component/ObjectReferences|GetgridManagerRef) 0)
          ;[1 1 1] Passes defined path to character. First Point character position last target
          (bind _pathpositions_2 (Default|GetCurrentPath (Variables|Component/ObjectReferences|GetgridManagerRef)))
          (Default|SetPath _output _pathpositions_2)
          (Default|MovetoGridPoint _output (Math|Vector|MakeVector (.x (Utilities|Array|Get(acopy) _pathpositions_2)) (.y (Utilities|Array|Get(acopy) _pathpositions_2)) (.z _returnvalue_2)) (Math|Vector|MakeVector (.x _returnvalue_2) (.y _returnvalue_2) (.z _returnvalue_2))))))))

(fn GetTurn
  (return (Variables|GameStates|GetcurrentTurn)))

(fn SetTurn
  (params (currentTurn :type TurnState%20Enum :default "NewEnumerator0"))
  (Variables|GameStates|SetcurrentTurn currentTurn))

(fn SetActiveSurvivor
  (params (BaseSurvivor :type BP%20Base%20Survivor%20Object%20Reference))
  (Variables|Component/ObjectReferences|SetActiveSurvivorRef BaseSurvivor))

(fn ResolveTurnLabels
  (switch Utilities|FlowControl|Switch|SwitchonTurnState (Variables|GameStates|GetcurrentTurn)
    (:NewEnumerator0
      (Variables|Labels|SetActiveTurnLabel (Variables|Labels|GetplayerTurnLabel)))
    (:NewEnumerator1
      (Variables|Labels|SetActiveTurnLabel (Variables|Labels|GetzombieTurnLabel)))))

(fn SetCanCharacterMove
  (params (canCharacterMove :type Boolean))
  (Variables|TurnData|SetcanCharacterMove canCharacterMove))

(fn ResolvePlayerTurns
  ;[1 1 1] Reduce Number of turns
  (bind _result (Math|Integer|DecrementInt (Variables|TurnData|GetnumSurvivorTurnsLeft))
    (:%20%20
      (if (not (> _result 0))
        ;[1 1 1] If number of turns is 0 or less end player turns
        (CallFunction|EndPlayerTurn)
        (Variables|TurnData|SetnumSurvivorTurnsLeft (Variables|TurnData|GetnumberOfSurvivors))))))

(fn ResolveZombieTurns
  ;[1 1 1] Reduce Number of turns
  (bind _result (Math|Integer|DecrementInt (Variables|TurnData|GetnumZombieTurnsLeft))
    (:%20%20
      (if (not (> _result 0))
        ;[1 1 1] If number of turns is 0 or less end player turns
        (CallFunction|EndZombieTurn)
        (Variables|TurnData|SetnumZombieTurnsLeft (Utilities|Array|Length (Variables|Characters|GetzombieRef)))))))

(fn StartAIActions
  (bind _output_get (Variables|TurnData|SetcurrentActiveZombieIndex 0))
  (Default|ZombieTakeTurn (Utilities|Array|Get(acopy) (Variables|Characters|GetzombieRef) _output_get)))

(fn TriggerNextZombieTurn
  (bind _result (Math|Integer|IncrementInt (Variables|TurnData|GetcurrentActiveZombieIndex))
    (:%20%20
      (if (!= (Utilities|Array|Get(acopy) (Variables|Characters|GetzombieRef) _result) 0)
        (Default|ZombieTakeTurn (Utilities|Array|Get(acopy) (Variables|Characters|GetzombieRef) _result))))))

(fn ResolveGame
  (if (> (Variables|Win/LossCondition|GetsurvivorsEscaped) 0)
    ;[1 1 1] If player ends game he survives to next stage
    (Development|PrintString "Win" true true "(R=0.000000,G=1.000000,B=0.204489,A=1.000000)")
    (Variables|Win/LossCondition|SetgameWon true)
    ;[1 1 1] Comment
    (Default|ToggleEscapeButton (Variables|Component/ObjectReferences|GetHudRef) false)
    (if (<= (Variables|TurnData|GetcurrentNumberOfSurvivors) 0)
      (Development|PrintString "end game" true true "(R=0.000000,G=1.000000,B=0.806052,A=1.000000)")
      (Default|CallOnEndGame)
      (Default|ToggleWinScreen (Variables|Component/ObjectReferences|GetHudRef) false)
      (Game|SetGamePaused true)
      (else
        (Development|PrintString "wait for player to end game" true true "(R=1.000000,G=0.921075,B=0.000000,A=1.000000)")))
    (elif (<= (Variables|TurnData|GetcurrentNumberOfSurvivors) 0)
      (Development|PrintString "Loss")
      (Variables|Win/LossCondition|SetgameWon false)
      (Development|PrintString "end game with loss icon")
      (Default|ToggleLossScreen (Variables|Component/ObjectReferences|GetHudRef) false))))

(fn EarlyEscape
  (Default|CallOnEndGame)
  (Default|ToggleWinScreen (Variables|Component/ObjectReferences|GetHudRef) false)
  (Game|SetGamePaused true)
  (Default|EndGame (Variables|Characters|GetzombieRef)))

(fn RetryLevel
  (bind _returnvalue (Game|GetCurrentLevelName true))
  (Game|OpenLevel(byName) (Utilities|String|StringToName _returnvalue)))