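; AudioManager Blueprint that centralizes playback of gameplay and UI sound effects, chosen by selection values.
; PlaySFX plays hurt or alarm sounds at a given location, while PlayUISound plays escape and level-fail sounds in 2D.
; Player and zombie hurt share one sound with a random pitch between MinPitch and MaxPitch to vary repeats.
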(event EventPlaySFX
  (params (actorLocation :type Vector :default "0, 0, 0") (soundEffect :type E_SoundEffects%20Enum :default "NewEnumerator0"))
  (CallFunction|PlaySFXatPoint soundEffect actorLocation))

(event EventPlayUISound
  (params (soundEffect :type E_SoundEffects%20Enum :default "NewEnumerator0"))
  (CallFunction|PlayUISFX soundEffect))

(fn ConstructionScript)

(fn PlaySFXatPoint
  (params (Selection :type E_SoundEffects%20Enum :default "NewEnumerator0") (Location :type Vector))
  (LocalVariables|Setpoint Location)
  (switch Utilities|FlowControl|Switch|SwitchonE_SoundEffects Selection
    (:NewEnumerator0
      (bind _returnvalue (CallFunction|GetRandomPitch :!label _label))
      (Audio|PlaySoundatLocation "/Game/Blueprints/Student/Assets/SFX/Hit_Hurt3.Hit_Hurt3" (LocalVariables|Getpoint) "0, 0, 0" 1.0 _returnvalue 0.0 0 0 0))
    (:NewEnumerator7
      (Audio|PlaySoundatLocation "/Game/Blueprints/Student/Assets/SFX/Car_alarm.Car_alarm" (LocalVariables|Getpoint) "0, 0, 0" 1.0 1.0 0.0 0 0 0))
    (:NewEnumerator8
      (goto _label))))

(fn GetRandomPitch
  (return (Math|Random|RandomFloatinRange (Variables|Default|GetminPitch) (Variables|Default|GetmaxPitch))))

(fn PlayUISFX
  (params (Selection :type E_SoundEffects%20Enum :default "NewEnumerator0"))
  (switch Utilities|FlowControl|Switch|SwitchonE_SoundEffects Selection
    (:NewEnumerator2
      (Audio|PlaySound2D "/Game/Blueprints/Student/Assets/SFX/Escaped.Escaped" 1.0 1.0 0.0 0 0))
    (:NewEnumerator4
      (Audio|PlaySound2D "/Game/Blueprints/Student/Assets/SFX/LossSfx.LossSfx" 1.0 1.0 0.0 0 0))))