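; Lootable car on the grid that survivors can search, with a failed loot attempt setting off a car alarm.
; Construction caches the grid and game managers and obstructs its cell; BeginPlay uses its cardinal yaw to spawn the car's other half in a neighbouring cell.
; The alarm notifies the game manager and propagates outward through each adjacent cell in its compass direction, up to AlarmRange steps.
; Attempts on an already looted car fail without an alarm.
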(event EventLoot
  (params (Interfacing%20Actor :type Actor%20Object%20Reference))
  (if (Variables|Default|GetisLooted)
    (bind _asbp_base_survivor (Utilities|Casting|CastToBP_BaseSurvivor Interfacing%20Actor))
    (Default|GiveLoot _asbp_base_survivor "NewEnumerator0" false)
    (else
      (bind _asbp_base_survivor_2 (Utilities|Casting|CastToBP_BaseSurvivor Interfacing%20Actor))
      (bind _lootsucess (CallFunction|LootActor))
      (if _lootsucess
        (Default|GiveLoot _asbp_base_survivor_2 (Variables|Default|GetcurrLoot) true)
        (else
          (Default|GiveLoot _asbp_base_survivor_2 "NewEnumerator0" false)
          (CallFunction|TriggerAlarm)
          (Class|GameEvents|CarAlarm(Message) (Variables|Default|GetGameManager%20Ref)))))))

(event EventBeginPlay
  (CallFunction|SpawnOtherHalf))

(fn ConstructionScript
  (|CallParentFunction)
  (CallFunction|Init))

(fn SpawnOtherHalf
  (bind _validrotation (CallFunction|ResolveRotation))
  (if _validrotation
    (bind (_cellcoordinate _validcell) (CallFunction|ResolveGridCoordinate))
    (if _validcell
      (Variables|Default|SetactorCoordinate _cellcoordinate)
      (bind (_spawncoord _rot) (CallFunction|ResolveOtherHalfSpawnPosition))
      (bind (_asbp_grid_floor _isvalid) (Default|GetCellfromCoordinate (Variables|Default|GetgridManagerRef) _spawncoord))
      (if _isvalid
        (Game|SpawnActorfromClass "/Game/Blueprints/Student/Blueprints/Looting/BP_CarHalfObstacle.BP_CarHalfObstacle_C" (Math|Transform|MakeTransform (Math|Vector|MakeVector (.x (Transformation|GetActorLocation _asbp_grid_floor)) (.y (Transformation|GetActorLocation _asbp_grid_floor)) (.z (Transformation|GetActorLocation))) _rot "1,1,1") "Undefined" 0 0)
        (else
          (Development|PrintString "coulnd't find cell from coordinate" true true "(R=1.000000,G=0.939989,B=0.000000,A=1.000000)" 5.0)))
      (else
        (Development|PrintString "no valid grid cell" true true "(R=1.000000,G=0.939989,B=0.000000,A=1.000000)" 5.0)))
    (else
      (Development|PrintString "bo valid rotation" true true "(R=1.000000,G=0.939989,B=0.000000,A=1.000000)" 5.0))))

(fn ResolveRotation
  (bind _output_get (LocalVariables|Setrotation (.yaw (Transformation|GetActorRotation))))
  (if (< _output_get 0.0)
    (LocalVariables|Setrotation (+ (LocalVariables|Getrotation) 3.6e+02)))
  (if (and (>= (LocalVariables|Getrotation) -1.0) (<= (LocalVariables|Getrotation) 1.0))
    (Variables|Default|SetcarOrientation "NewEnumerator0")
    (return true)
    (elif (and (>= (LocalVariables|Getrotation) 89.0) (<= (LocalVariables|Getrotation) 91.0))
      (Variables|Default|SetcarOrientation "NewEnumerator3")
      (return true)
      (elif (and (>= (LocalVariables|Getrotation) 179.0) (<= (LocalVariables|Getrotation) 181.0))
        (Variables|Default|SetcarOrientation "NewEnumerator1")
        (return true)
        (elif (and (>= (LocalVariables|Getrotation) 269.0) (<= (LocalVariables|Getrotation) 271.0))
          (Variables|Default|SetcarOrientation "NewEnumerator2")
          (return true)
          (else
            (return false)))))))

(fn ResolveGridCoordinate
  (bind (_cellexist _cellindex) (Default|GetCellfromWorldSpace (Variables|Default|GetgridManagerRef) (Transformation|GetActorLocation)))
  (if _cellexist
    (bind (_cellcoordinate _validcell) (Default|GetCellCoordinate (Variables|Default|GetgridManagerRef) _cellindex))
    (if _validcell
      (return _cellcoordinate true)
      (else
        (Development|PrintString "failed to resolve grid coordinate")
        (return "" false)))
    (else
      (Development|PrintString "failed to resolve grid coordinate")
      (return "" false))))

(fn ResolveOtherHalfSpawnPosition
  (bind _actorcoordinate (Variables|Default|GetactorCoordinate))
  (bind _actorcoordinate_2 (Variables|Default|GetactorCoordinate))
  (bind _actorcoordinate_3 (Variables|Default|GetactorCoordinate))
  (bind _actorcoordinate_4 (Variables|Default|GetactorCoordinate))
  (switch Utilities|FlowControl|Switch|SwitchonspawnOrientation (Variables|Default|GetcarOrientation)
    (:NewEnumerator0
      (bind _result (Math|Integer|DecrementInt (.y _actorcoordinate_3))
        (:%20%20
          (bind _output_get (LocalVariables|SetotherHalfCellCoord (Utilities|Struct|MakeInt2D (.x _actorcoordinate_3) _result)))
          (return _output_get "0,180.000000, 0"))))
    (:NewEnumerator1
      (bind _result_2 (Math|Integer|IncrementInt (.y _actorcoordinate))
        (:%20%20
          (bind _output_get_2 (LocalVariables|SetotherHalfCellCoord (Utilities|Struct|MakeInt2D (.x _actorcoordinate) _result_2)))
          (return _output_get_2 "0,0.000000, 0"))))
    (:NewEnumerator2
      (bind _result_3 (Math|Integer|DecrementInt (.x _actorcoordinate_4))
        (:%20%20
          (bind _output_get_3 (LocalVariables|SetotherHalfCellCoord (Utilities|Struct|MakeInt2D _result_3 (.y _actorcoordinate_4))))
          (return _output_get_3 "0,270.000000, 0"))))
    (:NewEnumerator3
      (bind _result_4 (Math|Integer|IncrementInt (.x _actorcoordinate_2))
        (:%20%20
          (bind _output_get_4 (LocalVariables|SetotherHalfCellCoord (Utilities|Struct|MakeInt2D _result_4 (.y _actorcoordinate_2))))
          (return _output_get_4 "0,90.000000, 0"))))))

(fn Init
  (bind _returnvalue (Actor|GetActorOfClass "/Game/Blueprints/Student/Blueprints/Grid/BP_GridManager.BP_GridManager_C"))
  (Variables|Default|SetGridManagerRef _returnvalue)
  (Class|GridEvents|ObstructActorCell(Message) (Variables|Default|GetgridManagerRef) self)
  (bind _returnvalue_2 (Actor|GetActorOfClass "/Game/Blueprints/Student/Blueprints/GameManagement/GameManager.GameManager_C"))
  (Variables|Default|SetGameManager%20Ref _returnvalue_2))

(fn TriggerAlarm
  (bind _cellcoordinate (CallFunction|ResolveGridCoordinate))
  (Variables|Default|SetactorCoordinate _cellcoordinate)
  (bind (_asbp_grid_floor _isvalid) (Default|GetCellfromCoordinate (Variables|Default|GetgridManagerRef) (Variables|Default|GetactorCoordinate)))
  (if _isvalid
    (bind _adjacentgridcells (Default|GetAdjacentCellArray _asbp_grid_floor))
    (for _array_element _adjacentgridcells
      (bind _cellcoordinate_2 (Default|GetGridCoordinate _array_element))
      (bind _alarmdir (CallFunction|ResolveAlarmDirections _cellcoordinate_2))
      (Default|SendAlarminDirection _array_element _alarmdir (Variables|Default|GetalarmRange) self))))

(fn ResolveAlarmDirections
  (params (coordinate :type Int%202D%20Structure))
  (bind _actorcoordinate (Variables|Default|GetactorCoordinate))
  (bind _actorcoordinate_2 (Variables|Default|GetactorCoordinate))
  (bind _actorcoordinate_3 (Variables|Default|GetactorCoordinate))
  (bind _actorcoordinate_4 (Variables|Default|GetactorCoordinate))
  (bind _actorcoordinate_5 (Variables|Default|GetactorCoordinate))
  (bind _actorcoordinate_6 (Variables|Default|GetactorCoordinate))
  (bind _actorcoordinate_7 (Variables|Default|GetactorCoordinate))
  (bind _actorcoordinate_8 (Variables|Default|GetactorCoordinate))
  (LocalVariables|SetcurrCellCoord coordinate)
  (if (and (== (.x _actorcoordinate_7) (.x (LocalVariables|GetcurrCellCoord))) (< (.y _actorcoordinate_7) (.y (LocalVariables|GetcurrCellCoord))))
    (return "NewEnumerator0")
    (elif (and (== (.x _actorcoordinate_8) (.x (LocalVariables|GetcurrCellCoord))) (> (.y _actorcoordinate_8) (.y (LocalVariables|GetcurrCellCoord))))
      (return "NewEnumerator1")
      (elif (and (> (.x _actorcoordinate) (.x (LocalVariables|GetcurrCellCoord))) (== (.y _actorcoordinate) (.y (LocalVariables|GetcurrCellCoord))))
        (return "NewEnumerator3")
        (elif (and (< (.x _actorcoordinate_2) (.x (LocalVariables|GetcurrCellCoord))) (== (.y _actorcoordinate_2) (.y (LocalVariables|GetcurrCellCoord))))
          (return "NewEnumerator2")
          (elif (and (> (.x _actorcoordinate_3) (.x (LocalVariables|GetcurrCellCoord))) (< (.y _actorcoordinate_3) (.y (LocalVariables|GetcurrCellCoord))))
            (return "NewEnumerator4")
            (elif (and (< (.x _actorcoordinate_4) (.x (LocalVariables|GetcurrCellCoord))) (< (.y _actorcoordinate_4) (.y (LocalVariables|GetcurrCellCoord))))
              (return "NewEnumerator5")
              (elif (and (> (.x _actorcoordinate_5) (.x (LocalVariables|GetcurrCellCoord))) (> (.y _actorcoordinate_5) (.y (LocalVariables|GetcurrCellCoord))))
                (return "NewEnumerator7")
                (elif (and (< (.x _actorcoordinate_6) (.x (LocalVariables|GetcurrCellCoord))) (> (.y _actorcoordinate_6) (.y (LocalVariables|GetcurrCellCoord))))
                  (return "NewEnumerator6"))))))))))