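; BP_CarHalfObstacle is a grid obstacle that stands in for part of a lootable car.
; On construction it finds the BP_GridManager in the level and has it obstruct the cell it occupies.
; Loot calls are forwarded to a parent car half, assigned through SetParentCar, so the parent handles the looting.
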(event EventLoot
  (params (Interfacing%20Actor :type Actor%20Object%20Reference))
  ;[1 1 1] Pass all loot information to car parent
  (Default|Loot (Variables|Default|GetparentCarHalf) Interfacing%20Actor))

(fn ConstructionScript
  (|CallParentFunction)
  (CallFunction|Init))

(fn SetParentCar
  (params (parentCarHAlf :type BP%20Car%20Lootable%20Object%20Reference))
  (Variables|Default|SetparentCarHalf parentCarHAlf))

(fn Init
  (bind _returnvalue (Actor|GetActorOfClass "/Game/Blueprints/Student/Blueprints/Grid/BP_GridManager.BP_GridManager_C"))
  (Variables|Default|SetGridManagerRef _returnvalue)
  (Class|GridEvents|ObstructActorCell(Message) (Variables|Default|GetgridManagerRef) self))