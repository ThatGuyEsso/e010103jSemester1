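; BP_BaseLootable is a base Blueprint for world objects that can be looted once.
; The construction script calls GenerateRandomLoot, which sets CurrLoot to one of the first two E_Loot entries at random.
; LootActor marks the object as looted on the first attempt, then rolls against LootSuccessRate and returns whether it succeeded, so a failed attempt also uses it up.
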(event EventBeginPlay)

(event Collision|EventActorBeginOverlap
  (params (OtherActor :type Actor%20Object%20Reference)))

(event EventTick
  (params (DeltaSeconds :type Float%20%28single-precision%29)))

(fn ConstructionScript
  (CallFunction|GenerateRandomLoot))

(fn GenerateRandomLoot
  (Variables|Default|SetcurrLoot (Utilities|Enum|ByteToEnumE_Loot (Math|Conversions|ToByte(Integer) (Math|Random|RandomIntegerinRange 0 1)))))

(fn LootActor
  (if (not (Variables|Default|GetisLooted))
    (Variables|Default|SetisLooted true)
    (if (<= (Math|Random|RandomFloat) (Variables|Default|GetlootSuccessRate))
      (return true)
      (else
        (return false)))))