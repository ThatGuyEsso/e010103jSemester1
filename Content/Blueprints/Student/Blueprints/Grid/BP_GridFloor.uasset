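; BP_GridFloor is one grid cell that tracks active, obstructed, exit, target and character state, mostly showing it through material swaps.
; It gathers its eight-way neighbours from the grid manager by coordinate.
; Paths grow greedily cell to cell, by world location or coordinate: each activates the nearest free neighbour, reports its location to the manager and recurses with fewer steps.
; The FindNewPath fallback for blocked cells is unfinished, with disconnected index selection.
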(event Custom|Deactivate
  ;[1 1 1] Deactivate cell
  (if (not (Variables|States|GetisObstructed))
    (Rendering|Material|SetMaterial (Variables|Default|GetMesh) 0 (Variables|Materials|GetOffMaterial))
    (Variables|States|SetisActive false)
    ;[1 1 1] If exist celll make sure it looks like it
    (if (Variables|States|GetisExit)
      (CallFunction|CreateExitCell))))

(event Custom|UnObstruct
  ;[1 1 1] UnObstruct Cell
  (Rendering|Material|SetMaterial (Variables|Default|GetMesh) 0 (Variables|Materials|GetOffMaterial))
  (Variables|States|SetisObstructed false))

(event Custom|Activate
  ;[1 1 1] Activate cell
  (Rendering|Material|SetMaterial (Variables|Default|GetMesh) 0 (Variables|Materials|GetOnMaterial))
  (Variables|States|SetisActive true)
  ;[1 1 1] If exist celll make sure it looks like it
  (if (Variables|States|GetisExit)
    (CallFunction|CreateExitCell)))

(event Custom|MakeObstucted
  ;[1 1 1] Obstuct Cell
  (if (not (Variables|States|GetisExit)) ; Exit can't be obstructed
    (Rendering|Material|SetMaterial (Variables|Default|GetMesh) 0 (Variables|Materials|GetobstructedMaterial))
    (Variables|States|SetisObstructed true)))

(event Custom|CreateExitCell
  ;[1 1 1] Make cell Exit cell
  (Rendering|Material|SetMaterial (Variables|Default|GetMesh) 0 (Variables|Materials|GetexitMaterial))
  (Variables|States|SetisExit true))

(event EventBeginPlay
  (if (Variables|States|GetisExit)
    (CallFunction|CreateExitCell)))

(fn ConstructionScript)

(fn GetIsActive
  (return (Variables|States|GetisActive)))

(fn SetHasCharacter
  (params (hasCharacter :type Boolean))
  (Variables|States|SethasCharacter hasCharacter))

(fn GetHasCharacter
  (return (Variables|States|GethasCharacter)))

(fn GetIsObstructed
  (return (Variables|States|GetisObstructed)))

(fn SetIsObstructed
  (params (isObstructed :type Boolean))
  (Variables|States|SetisObstructed isObstructed))

(fn GetAllAdjacentCells
  (bind _cellcoordinate (Variables|Actor/CompoenentRefs|GetcellCoordinate))
  ;[1 1 1] Get own cell coordinate
  (bind _cellcoordinate_2 (CallFunction|GetGridCoordinate))
  ;[1 1 1] Set coordinate limit of left  most neighbour, and right most neighbour + the same for top and bottom
  (bind _output_get (LocalVariables|SetcellPosition _cellcoordinate_2))
  (LocalVariables|SetminX (- (.x _output_get) 1))
  (LocalVariables|SetmaxX (+ (.x (LocalVariables|GetcellPosition)) 1))
  (LocalVariables|SetminY (- (.y (LocalVariables|GetcellPosition)) 1))
  (LocalVariables|SetmaxY (+ (.y (LocalVariables|GetcellPosition)) 1))
  ;[1 1 1] Cycle through from left bottom to right top respective to cell coordinate
  (for _index (range (LocalVariables|GetminX) (LocalVariables|GetmaxX))
    (for _index_2 (range (LocalVariables|GetminY) (LocalVariables|GetmaxY))
      ;[1 1 1] Get cell at that postion from grid manager
      (bind _asbp_grid_floor (Default|GetCellfromCoordinate (Variables|Actor/Compoenentrefs|GetGridManagerRef) (Utilities|Struct|MakeInt2D _index _index_2)))
      ;[1 1 1] Check if cell exist (I.E is this cell on a boundary)
      (if (!= _asbp_grid_floor 0)
        ;[1 1 1] If cell is not self and it exist add to list of adjacent cells
        (if (not (and (== (.x (Variables|BP_GridFloor_C|GetcellCoordinate _asbp_grid_floor)) (.x _cellcoordinate)) (== (.y (Variables|BP_GridFloor_C|GetcellCoordinate _asbp_grid_floor)) (.y _cellcoordinate))))
          (Utilities|Array|Add (Variables|Actor/CompoenentRefs|GetadjacentGridCells) _asbp_grid_floor))))))

(fn ActivateClosesCelltoPoint
  (params (location :type Vector) (stepsLeft :type Integer))
  (if (Math|Vector|Equal(Vector) location (Transformation|GetActorLocation) 0.5)
    (CallFunction|SetIsTarget true)
    (else
      (bind _output_get (LocalVariables|SetnewNumStepsLeft stepsLeft))
      (if (> _output_get 0)
        (LocalVariables|SetshortestDistance (Math|Vector|VectorLengthXY (- location (Transformation|GetActorLocation))))
        (for (_array_element _array_index) (Variables|Actor/CompoenentRefs|GetadjacentGridCells)
          (bind _isfree (CallFunction|IsCellFree _array_element))
          (if _isfree
            (if (< (Math|Vector|VectorLengthXY (- location (Transformation|GetActorLocation _array_element))) (LocalVariables|GetshortestDistance))
              ;[1 1 1] If grid floor is closer calculate new shortest distance and get index
              (LocalVariables|SetShortestIndex _array_index)
              (LocalVariables|SetshortestDistance (Math|Vector|VectorLengthXY (- location (Transformation|GetActorLocation _array_element)))))))
        ;[1 1 1] Check if cell isn't already active or obstructed (Must be the final ponint if it is active)
        (bind _output_get_2 (LocalVariables|SetcurrentCell (Utilities|Array|Get(acopy) (Variables|Actor/CompoenentRefs|GetadjacentGridCells) (LocalVariables|GetShortestIndex))))
        (bind _isobstructed (CallFunction|GetIsObstructed _output_get_2))
        (if _isobstructed
          (CallFunction|FindNewPath location (LocalVariables|GetnewNumStepsLeft) :!label _label)
          (else
            (bind _hascharacter (CallFunction|GetHasCharacter (LocalVariables|GetcurrentCell)))
            (if _hascharacter
              (goto _label)
              (else
                (bind _istarget (CallFunction|GetIsTarget (LocalVariables|GetcurrentCell)))
                ;[1 1 1] If false activate  cell and tell it to the same search
                (if _istarget
                  (Default|AddtoPathPoints (Variables|Actor/Compoenentrefs|GetGridManagerRef) (Transformation|GetActorLocation (LocalVariables|GetcurrentCell)))
                  (else
                    (bind _isactive (CallFunction|GetIsActive (LocalVariables|GetcurrentCell)))
                    (if _isactive
                      (CallFunction|FindNewPath location)
                      (else
                        (CallFunction|Activate (LocalVariables|GetcurrentCell))
                        (if (!= (Variables|Actor/Compoenentrefs|GetGridManagerRef) 0)
                          (Math|Integer|DecrementInt (LocalVariables|GetnewNumStepsLeft)
                            (:%20%20
                              (Default|AddtoPathPoints (Variables|Actor/Compoenentrefs|GetGridManagerRef) (Transformation|GetActorLocation (LocalVariables|GetcurrentCell)))
                              (CallFunction|ActivateClosesCelltoPoint (LocalVariables|GetcurrentCell) location (LocalVariables|GetnewNumStepsLeft)))))))))))))))))

(fn FindNewPath
  (params (targetPos :type Vector) (stepsLeft :type Integer))
  (bind _adjacentgridcells (Variables|Actor/CompoenentRefs|GetadjacentGridCells))
  (bind _newpathindex (LocalVariables|GetnewPathIndex))
  (bind _output (Utilities|Array|Get(acopy) _adjacentgridcells _newpathindex))
  (if (Math|Vector|Equal(Vector) targetPos (Transformation|GetActorLocation) 0.5)
    (CallFunction|SetIsTarget true)
    (Development|PrintString "Hello")
    (else
      (LocalVariables|SetnewStepsLeft stepsLeft)
      (if (> stepsLeft 0)
        (LocalVariables|SettargetPosition targetPos)
        (for (_array_element _array_index) (Variables|Actor/CompoenentRefs|GetadjacentGridCells)
          ;[1 1 1] Checks if cells are active ore obstructed
          (bind _isobstructed (CallFunction|GetIsObstructed _array_element))
          (if (not _isobstructed)
            (bind _isactive (CallFunction|GetIsActive _array_element))
            (if (not _isactive)
              (bind _hascharacter (CallFunction|GetHasCharacter _array_element))
              (if (not _hascharacter)
                (Utilities|Array|Add (LocalVariables|GetpossibleIndices) _array_index)
                (LocalVariables|SetSuccess true)))))
        (Utilities|FlowControl|Sequence
          (:then_0
            (if (LocalVariables|GetSuccess)
              (for (_array_element_2 _array_index_2) (LocalVariables|GetpossibleIndices)
                (if (not (== _array_index_2 0))
                  (if (< (Math|Vector|VectorLengthXY (- (LocalVariables|GettargetPosition) (Transformation|GetActorLocation (Utilities|Array|Get(acopy) (Variables|Actor/CompoenentRefs|GetadjacentGridCells) _array_element_2)))) 0.0)
                    _)))
              (else
                (Development|PrintString "Locked in"))))
          (:then_1
            (if (LocalVariables|GetSuccess)
              (bind _istarget (CallFunction|GetIsTarget _output))
              (if _istarget
                (Default|AddtoPathPoints (Variables|Actor/Compoenentrefs|GetGridManagerRef) (Transformation|GetActorLocation _output))
                (else
                  (Math|Integer|DecrementInt (LocalVariables|GetnewStepsLeft)
                    (:%20%20
                      (CallFunction|Activate _output)
                      (Default|AddtoPathPoints (Variables|Actor/Compoenentrefs|GetGridManagerRef) (Transformation|GetActorLocation _output))
                      (CallFunction|ActivateClosesCelltoPoint _output (LocalVariables|GettargetPosition)))))))))))))

(fn GetIsTarget
  (return (Variables|States|GetisTarget)))

(fn SetIsTarget
  (params (isTarget :type Boolean))
  (Variables|States|SetisTarget isTarget))

(fn GetClosesCelltoPoint
  (params (point :type Vector))
  (LocalVariables|SetshortestDistance (Math|Vector|VectorLengthXY (- point (Transformation|GetActorLocation))))
  (for (_array_element _array_index) (Variables|Actor/CompoenentRefs|GetadjacentGridCells)
    (bind _isfree (CallFunction|IsCellFree _array_element))
    (if _isfree
      (if (< (Math|Vector|VectorLengthXY (- point (Transformation|GetActorLocation))) (LocalVariables|GetshortestDistance))
        (LocalVariables|SetShortestIndex _array_index))))
  (return (Utilities|Array|Get(acopy) (Variables|Actor/CompoenentRefs|GetadjacentGridCells) (LocalVariables|GetShortestIndex))))

(fn GetAdjacentCellArray
  (return (Variables|Actor/CompoenentRefs|GetadjacentGridCells)))

(fn GetIsExit
  (return (Variables|States|GetisExit)))

(fn GetGridCoordinate
  (return (Variables|Actor/CompoenentRefs|GetcellCoordinate)))

(fn SetGridCoordinate
  (params (Cell%20Coordinate%20X :type Integer) (Cell%20Coordinate%20Y :type Integer))
  (Variables|Actor/CompoenentRefs|SetcellCoordinate (Utilities|Struct|MakeInt2D Cell%20Coordinate%20X Cell%20Coordinate%20Y)))

(fn SetGridManager
  (params (GridManagerRef :type BP%20Grid%20Manager%20Object%20Reference))
  (Variables|Actor/Compoenentrefs|SetGridManagerRef GridManagerRef))

(fn SetAboveActor
  (params (aboveActor :type Actor%20Object%20Reference))
  (Variables|Actor/CompoenentRefs|SetaboveActor aboveActor))

(fn RemoveAboveActor
  (Variables|Actor/CompoenentRefs|SetaboveActor 0))

(fn GetAboveActor
  (return (Variables|Actor/CompoenentRefs|GetaboveActor)))

(fn GetClosesAdjacentCelltoPoint
  (params (targetCellCoordinate :type Int%202D%20Structure) (numberOfstepsLeft :type Integer))
  (bind _cellcoordinate (Variables|Actor/CompoenentRefs|GetcellCoordinate))
  (LocalVariables|SetStepsleft numberOfstepsLeft)
  (if (> numberOfstepsLeft 0)
    ;[1 1 1] Check if target is current cell based cell coordinate
    (bind _output_get (LocalVariables|SettargetCoord targetCellCoordinate))
    (Development|PrintString (Utilities|String|ToString(Integer) (.x _output_get)))
    (Development|PrintString (Utilities|String|ToString(Integer) (.y _output_get)))
    (if (and (== (.x _output_get) (.x _cellcoordinate)) (== (.y _output_get) (.y _cellcoordinate)))
      ;[1 1 1] If cell coordinates match, add this to point and stop
      (CallFunction|SetIsTarget true)
      (CallFunction|AddPointtoPath (Transformation|GetActorLocation))
      (CallFunction|Activate)
      (else
        ;[1 1 1] Calculate inital shortest distance
        (bind _distance (CallFunction|GetDistanceBtwnCells (Variables|Actor/CompoenentRefs|GetcellCoordinate) (LocalVariables|GettargetCoord)))
        (bind _output_get_2 (LocalVariables|SetshortestDistance _distance))
        (Development|PrintString (Utilities|String|ToString(Float) _output_get_2))
        (for (_array_element _array_index) (Variables|Actor/CompoenentRefs|GetadjacentGridCells)
          ;[1 1 1] Check if cell is free and get closes index of cell to target
          (bind _isfree (CallFunction|IsCellFree _array_element))
          (if _isfree
            (bind _cellcoordinate_2 (CallFunction|GetGridCoordinate _array_element))
            (bind _distance_2 (CallFunction|GetDistanceBtwnCells _cellcoordinate_2 (LocalVariables|GettargetCoord)))
            (if (< _distance_2 (LocalVariables|GetshortestDistance))
              (LocalVariables|SetclosestIndex _array_index)
              (LocalVariables|SetfoundCell true)
              (else
                (LocalVariables|SetfoundCell false)))
            (else
              (LocalVariables|SetfoundCell false))))
        ;[1 1 1] Checks if cell found
        (if (LocalVariables|GetfoundCell)
          ;[1 1 1] Add to path and decrement steps left
          (CallFunction|AddPointtoPath (Transformation|GetActorLocation (Utilities|Array|Get(acopy) (Variables|Actor/CompoenentRefs|GetadjacentGridCells) (LocalVariables|GetclosestIndex))))
          (CallFunction|Activate (Utilities|Array|Get(acopy) (Variables|Actor/CompoenentRefs|GetadjacentGridCells) (LocalVariables|GetclosestIndex)))
          (bind _result (Math|Integer|DecrementInt (LocalVariables|GetStepsleft))
            (:%20%20
              (CallFunction|GetClosesAdjacentCelltoPoint (Utilities|Array|Get(acopy) (Variables|Actor/CompoenentRefs|GetadjacentGridCells) (LocalVariables|GetclosestIndex)) (LocalVariables|GettargetCoord) _result)))
          (else
            (Development|PrintString "nopath found")
            ;[1 1 1] If no path found remain
            (CallFunction|AddPointtoPath (Transformation|GetActorLocation))))))))

(fn AddPointtoPath
  (params (pathPoint :type Vector%20%28by%20ref%29))
  (Default|AddtoPathPoints (Variables|Actor/Compoenentrefs|GetGridManagerRef) pathPoint))

(fn GetDistanceBtwnCells
  (params (cellPositionA :type Int%202D%20Structure) (cellPositionB :type Int%202D%20Structure))
  ;[1 1 1] Calculate vector to point
  (LocalVariables|SetvectorToPoint (Utilities|Struct|MakeInt2D (- (.x cellPositionB) (.x cellPositionA)) (- (.y cellPositionB) (.y cellPositionA))))
  (return (Math|Float|Sqrt (+ (Math|Conversions|ToFloat(Integer) (.x (LocalVariables|GetvectorToPoint))) (Math|Conversions|ToFloat(Integer) (.y (LocalVariables|GetvectorToPoint)))))))

(fn IsCellFree
  (bind _isobstructed (CallFunction|GetIsObstructed 0))
  (if _isobstructed
    (return false)
    (else
      (bind _isactive (CallFunction|GetIsActive 0))
      (if _isactive
        (return false)
        (else
          (bind _hascharacter (CallFunction|GetHasCharacter 0))
          (if _hascharacter
            (return false)
            (else
              (return true))))))))

(fn SetOffMaterial
  (params (OffMaterial :type Material%20Interface%20Object%20Reference))
  (bind _output_get (Variables|Materials|SetOffMaterial OffMaterial))
  (Rendering|Material|SetMaterial (Variables|Default|GetMesh) 0 _output_get)
  (Development|PrintString "default grid material has been applied"))