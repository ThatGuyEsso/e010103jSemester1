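; GridMap Blueprint that holds a 2D grid as a flat array of map-data structs, with CellSize giving the cell count on each axis.
; On BeginPlay it sizes the array to X times Y, builds coordinates in X-major order and copies each into the matching cell's CellCoordinate.
; GetCellSize exposes the dimensions, while the GenerateMap event and construction script are empty.
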(event Custom|GenerateMap)

(event EventBeginPlay
  (CallFunction|AssignCellCoordinates))

(fn ConstructionScript)

(fn GetCellSize
  (return (Variables|Default|GetcellSize)))

(fn AssignCellCoordinates
  (bind _cellsize (Variables|Default|GetcellSize))
  (bind _cellsize_2 (Variables|Default|GetcellSize))
  (Utilities|FlowControl|Sequence
    (:then_0
      (Utilities|Array|Resize (Variables|Default|GetgridMap) (* (.x _cellsize) (.y _cellsize)))
      (for _index (range 0 (- (.x _cellsize_2) 1))
        (for _index_2 (range 0 (- (.y _cellsize_2) 1))
          (Utilities|Array|Add (LocalVariables|Getcoords) (Utilities|Struct|MakeInt2D _index _index_2)))))
    (:then_1
      (for (_ _array_index) (Variables|Default|GetGridMap)
        (Utilities|Struct|SetmembersinmapData (Utilities|Array|Get(acopy) (Variables|Default|GetGridMap) _array_index) (Utilities|Array|Get(acopy) (LocalVariables|Getcoords) _array_index))))))