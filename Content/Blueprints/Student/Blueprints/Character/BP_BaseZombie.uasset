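; Base zombie character for a turn-based grid game, moving to random cells on its turn.
; Each turn it samples points within WalkRange until one lands on a grid cell, then submits that cell to the grid manager, repeating if the location is rejected.
; Actions reset when the game manager signals the player's turn has ended; once they run out, it triggers the next zombie and resolves zombie turns.
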(event Custom|ZombieTake%20Turn
  (bind _cellindex (CallFunction|GetRandomPositionAroundCharacter 0.0 (Variables|Default|GetWalkRange)))
  (Default|ZombieFoundMoveLocation (Variables|Default|GetGridManagerRef) self _cellindex))

(event Custom|OnTurnStart
  (CallFunction|ResetActionsLeft))

(event EventZombieMoveLocationIsNotValid
  (CallFunction|ZombieTakeTurn))

(event EventBeginPlay
  (EventDispatchers|BindEventtoEventEndPlayerTurn (Variables|Default|GetGameMangerRef) (delegate Custom|OnTurnStart)))

(fn ConstructionScript
  (|CallParentFunction))

(fn GetRandomPositionAroundCharacter
  (params (minDistance :type Float%20%28single-precision%29) (maxDistance :type Float%20%28single-precision%29))
  (bind _gridmanagerref (Variables|Default|GetGridManagerRef))
  (LocalVariables|Setextents maxDistance)
  (bind _output_get (LocalVariables|Setpoint (Math|Random|RandomPointinBoundingBox (Transformation|GetActorLocation) (Math|Vector|MakeVector maxDistance maxDistance 5e+01))))
  (bind (_cellexist _cellindex) (Default|GetCellfromWorldSpace (Variables|Default|GetGridManagerRef) _output_get))
  (if _cellexist
    (return _cellindex)
    (else
      (while (Math|Boolean|NotEqual(Boolean) (LocalVariables|GetCell%20exist) true)
        (bind _output_get_2 (LocalVariables|Setpoint (Math|Random|RandomPointinBoundingBox (Transformation|GetActorLocation) (Math|Vector|MakeVector (LocalVariables|Getextents) (LocalVariables|Getextents) 5e+01))))
        (bind _cellexist_2 (Default|GetCellfromWorldSpace _gridmanagerref _output_get_2))
        (LocalVariables|SetCell%20exist _cellexist_2))
      (bind _cellindex_2 (Default|GetCellfromWorldSpace _gridmanagerref (LocalVariables|Getpoint)))
      (return _cellindex_2))))

(fn EndAction
  (bind _gamemangerref (Variables|Default|GetGameMangerRef))
  ;[1 1 1] If character has no actions left character needs to tell game manager that their individual turn has ended(Note other character on it team might still have more turns left)
  (Math|Integer|DecrementInt (Variables|Default|GetactionsLeft)
    (:%20%20
      (if (not (> (Variables|Default|GetactionsLeft) 0))
        (Default|TriggerNextZombieTurn _gamemangerref)
        (Default|ResolveZombieTurns _gamemangerref)))))