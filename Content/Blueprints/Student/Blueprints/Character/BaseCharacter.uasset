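; Base grid character for a turn-based game that moves cell by cell along a stored path and marks which floor cell it occupies.
; Init registers its starting cell and fills its action count, using manager references found in the construction script.
; MoveToGridPoint lerps location on a timeline while tracking the current cell.
; Each finished step clears that cell's highlight and target, then chains to the next point or ends the player turn.
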(event Custom|MoveToGridPoint
  (params (newPoint :type Vector) (startPoint :type Vector))
  (bind _returnvalue (Transformation|GetActorLocation))
  (bind _gridmanagerref (Variables|Component/ObjectRefs|GetGridManagerRef))
  (bind _gridmanagerref_2 (Variables|Component/ObjectRefs|GetGridManagerRef))
  (bind _pathentry (Variables|Pathing|GetpathEntry))
  (bind _currentpathindex (Variables|Pathing|GetcurrentPathIndex))
  (bind _output (Utilities|Array|Get(acopy) _pathentry _currentpathindex))
  (CallFunction|ToggleCellPosition (Variables|Pathing|GetcurrentGridIndex) false)
  (bind _alpha (Timeline|MoveTimeLine PlayFromStart)
    (:Update
      (Variables|CharacterState|SetisMoving true)
      (Transformation|SetActorLocation (Math|Vector|Lerp(Vector) startPoint newPoint _alpha) false false)
      (bind (_cellexist _cellindex) (Default|GetCellfromWorldSpace _gridmanagerref_2 (Transformation|GetActorLocation)))
      (if _cellexist
        (Variables|Pathing|SetcurrentGridIndex _cellindex)))
    (:Finished
      (Variables|CharacterState|SetisMoving false)
      (if (!= _gridmanagerref 0)
        (bind (_cellexist_2 _cellindex_2) (Default|GetCellfromWorldSpace _gridmanagerref (Transformation|GetActorLocation)))
        (if _cellexist_2
          (Default|ToggleGridFloor _gridmanagerref_2 false _cellindex_2)
          (Default|ToggleTarget _gridmanagerref_2 (Variables|Pathing|GetcurrentGridIndex) false)
          (CallFunction|ToggleCellPosition _cellindex_2 true)
          (Math|Integer|IncrementInt (Variables|Pathing|GetcurrentPathIndex)
            (:%20%20
              (if (< (Variables|Pathing|GetcurrentPathIndex) (Utilities|Array|Length (Variables|Pathing|GetpathEntry)))
                (CallFunction|MovetoGridPoint (Math|Vector|MakeVector (.x _output) (.y _output) (.z _returnvalue)) (Math|Vector|MakeVector (.x _returnvalue) (.y _returnvalue) (.z _returnvalue)))
                (else
                  (Default|EndPlayerTurn (Variables|Component/ObjectRefs|GetGameMangerRef)))))))))))

(event EventBeginPlay
  (CallFunction|Init))

(fn ConstructionScript
  (bind _returnvalue (Actor|GetActorOfClass "/Game/Blueprints/Student/Blueprints/Grid/GridManager.GridManager_C"))
  (Variables|Default|SetgridManagerRef _returnvalue)
  (bind _returnvalue_2 (Actor|GetActorOfClass "/Game/Blueprints/Student/Blueprints/GameManagement/GameManager.GameManager_C"))
  (Variables|Component/ObjectRefs|SetGameMangerRef _returnvalue_2))

(fn ToggleCellPosition
  (params (GridCellIndex :type Integer) (hasCharacter :type Boolean))
  (bind _gridmanagerref (Variables|Component/ObjectRefs|GetGridManagerRef))
  ;[1 1 1] Null ptr check
  (if (!= _gridmanagerref 0)
    (bind _asgrid_floor (Utilities|Casting|CastToGridFloor (Utilities|Array|Get(acopy) (Variables|/Game/Blueprints/Student/Blueprints/Grid/GridManager.GridManager_C|GetGridFloor _gridmanagerref) GridCellIndex)))
    (Default|SetHasCharacter _asgrid_floor hasCharacter)))

(fn SetPath
  (params (pathPoints :type Array%20of%20Vectors))
  (Variables|Pathing|SetcurrentPathIndex 0)
  (Utilities|Array|Clear (Variables|Pathing|GetpathEntry))
  (for _array_element pathPoints
    (Utilities|Array|Add (Variables|Pathing|GetpathEntry) _array_element)))

(fn Init
  (bind (_cellexist _cellindex) (Default|GetCellfromWorldSpace (Variables|Component/ObjectRefs|GetGridManagerRef) (Transformation|GetActorLocation)))
  (if _cellexist
    (bind _output_get (Variables|Pathing|SetcurrentGridIndex _cellindex))
    (CallFunction|ToggleCellPosition _output_get true)
    (Variables|settings|SetcurrentNumberOfActions (Variables|settings|GetmaxNumberOfActions))))