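; BP_BaseSurvivor is the base survivor character, a selectable unit with a limited number of actions per turn in a turn-based game with zombies.
; It binds to the game manager's end-of-zombie-turn event to reset its remaining actions.
; Selection requires actions left and swaps the Cube's material to show the selected state.
; Ending an action runs the parent logic, then deselects the survivor and restores its original material.
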(event Custom|Select%20Character
  (if (> (Variables|Default|GetactionsLeft) 0)
    ;[1 1 1] Select Character
    (Rendering|Material|SetMaterial (Variables|Default|GetCube) 0 (Variables|Material|GetOnMaterial))
    (Variables|CharacterState|SetisSelected true)))

(event Custom|UnSelect%20Character
  ;[1 1 1] Unselect Character
  (Rendering|Material|SetMaterial (Variables|Default|GetCube) 0 (Variables|Material|GetOffMaterial))
  (Variables|CharacterState|SetisSelected false))

(event Custom|OnTurnStart
  (CallFunction|ResetActionsLeft))

(event EventBeginPlay
  ;[1 1 1] Set Initial material
  (CallFunction|Init)
  (Variables|Material|SetOffMaterial (Utilities|Array|Get(acopy) (Rendering|Material|GetMaterials (Variables|Default|GetCube))))
  (Variables|Default|SetactionsLeft (Variables|Default|GetMaxActions))
  (EventDispatchers|BindEventtoEventEndZombieTurn (Variables|Default|GetGameMangerRef) (delegate Custom|OnTurnStart)))

(fn ConstructionScript
  (|CallParentFunction))

(fn GetIsSelected
  (return (Variables|CharacterState|GetisSelected)))

(fn EndAction
  (|CallParentFunction)
  (CallFunction|UnSelectCharacter))