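; Player controller that turns mouse clicks into cell selections on a grid, apparently to drive grid-based movement.
; On BeginPlay it caches references to the B_AdvCharacter and GridManager actors found in the level.
; A left click deprojects the cursor into a Visibility line trace and passes any impact point to the GridManager's OnCellSelection.
; A missed trace only prints a debug message.
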(event EventBeginPlay
  ;[1 1 1] Cache actor references
  (bind _returnvalue (Actor|GetActorOfClass "/Game/Blueprints/B_AdvCharacter.B_AdvCharacter_C"))
  (Variables|Default|SetCharacterRef _returnvalue)
  (bind _returnvalue_2 (Actor|GetActorOfClass "/Game/Blueprints/Student/Blueprints/Grid/GridManager.GridManager_C"))
  (Variables|Default|SetGridMangerRef _returnvalue_2))

(event Input|MouseEvents|LeftMouseButton
  (params (Key :type Key%20Structure :default "None"))
  (:Pressed
    ;[1 1 1] Shoots Raycast to mouse position and triggers grid movement
    (bind (_point _istherehit) (CallFunction|TracetoMousePosition))
    (if _istherehit
      (Default|OnCellSelection (Variables|Default|GetGridMangerRef) _point))))

(fn ConstructionScript)

(fn TracetoMousePosition
  (bind _returnvalue (Game|GetPlayerController 0))
  (bind (_worldlocation _worlddirection) (Game|Player|ConvertMouseLocationToWorldSpace _returnvalue))
  (bind (_outhit _returnvalue_2) (Collision|LineTraceByChannel _worldlocation (+ _worldlocation (* _worlddirection (Variables|Default|GetTraceLength))) "TraceTypeQuery1" false 0 "None"))
  (if _returnvalue_2
    (return (.ImpactPoint (Collision|BreakHitResult _outhit)) _returnvalue_2)
    (else
      (Development|PrintString "Hit Nothing"))))